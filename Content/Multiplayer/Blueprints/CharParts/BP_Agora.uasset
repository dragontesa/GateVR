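; BP_Agora wraps the Agora RTC SDK to provide multiplayer voice chat for the VR game.
; InitVoice creates the engine and applies the saved mic setting, while other functions handle channel join and leave, release, muting, volume indication and an echo preset.
; Device selection searches for Oculus Virtual Audio devices by name.
; Spatial audio helpers feed VR camera and remote player positions to Agora, but InitVoice's InitSpatialVoice call is disconnected.
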(event EventBeginPlay)

(event Collision|EventActorBeginOverlap
  (params (OtherActor :type Actor%20Object%20Reference)))

(event EventTick
  (params (DeltaSeconds :type Float%20%28single-precision%29)))

(fn ConstructionScript)

(fn InitVoice
  (bind _returnvalue (Game|GetPlayerController 0))
  (Variables|Default|GetRtcEngine_Ref
    (:then)
    (:else
      (bind _returnvalue_2 (Game|ConstructObjectfromClass _returnvalue "/Script/AgoraPlugin.IRtcEngineEventHandler"))
      (bind _output_get (Variables|Default|SetRtcEngine_EventHandle _returnvalue_2))
      (bind _returnvalue_3 (Game|ConstructObjectfromClass _returnvalue "/Script/AgoraPlugin.AgoraRtcEngine"))
      (bind _output_get_2 (Variables|Default|SetRtcEngine_Ref _returnvalue_3))
      (Class|AgoraRtcEngine|Initialize _output_get_2 (Utilities|Struct|MakeRtcEngineContext "13b44aa785094489a54fb06ee22d45c5" _output_get 0 "" "CHANNEL_PROFILE_COMMUNICATION" "AUDIO_SCENARIO_DEFAULT" false "HIGH"))
      (Utilities|FlowControl|Sequence
        (:then_0
          (bind _returnvalue_4 (Class|AgoraRtcEngine|QueryInterface (Variables|Default|GetRtcEngine_Ref) "AGORA_IID_AUDIO_DEVICE_MANAGER"))
          (bind _asiaudio_device_manager (Utilities|Casting|CastToIAudioDeviceManager _returnvalue_4))
          (Variables|Default|SetAudioDeviceManager _asiaudio_device_manager))
        (:then_1
          (bind _returnvalue_5 (SaveGame|LoadGamefromSlot "DisplayMenu"))
          (bind _assave_display_menu (Utilities|Casting|CastToSave_DisplayMenu _returnvalue_5))
          (CallFunction|MuteVoice (not (Variables|/Game/XHUD/DisplayMenu/Save_DisplayMenu.Save_DisplayMenu_C|GetIsMic_On _assave_display_menu))))))))

(fn InitSpatialVoice
  (bind _returnvalue (Class|AgoraRtcEngine|QueryInterface (Variables|Default|GetRtcEngine_Ref) "AGORA_IID_LOCAL_SPATIAL_AUDIO"))
  (bind _asilocal_spatial_audio_engine (Utilities|Casting|CastToILocalSpatialAudioEngine _returnvalue))
  (bind _output_get (Variables|Default|SetLocalSpatial _asilocal_spatial_audio_engine))
  (|SetBy-RefVar (stale _config) (Utilities|Struct|MakeLocalSpatialAudioConfig (Variables|Default|GetRtcEngine_Ref)))
  (bind _config (Class|ILocalSpatialAudioEngine|Initialize _output_get))
  (Class|ILocalSpatialAudioEngine|SetAudioRecvRange (Variables|Default|GetLocalSpatial) 2e+04)
  (Class|ILocalSpatialAudioEngine|SetDistanceUnit (Variables|Default|GetLocalSpatial) 0.01))

(fn ReleaseVoice
  (bind _rtcengine_ref (Variables|Default|GetRtcEngine_Ref)
    (:then
      (Class|AgoraRtcEngine|LeaveChannel _rtcengine_ref (Utilities|Struct|MakeLeaveChannelOptions "AGORA_NULL_VALUE" "AGORA_NULL_VALUE" "AGORA_NULL_VALUE"))
      (Class|AgoraRtcEngine|UnregisterEventHandler _rtcengine_ref (Variables|Default|GetRtcEngine_EventHandle))
      (Class|AgoraRtcEngine|Release _rtcengine_ref true)
      (Variables|Default|SetRtcEngine_EventHandle 0)
      (Variables|Default|SetRtcEngine_Ref 0))
    (:else)))

(fn JoinVoiceChannel
  (params (channelId :type String))
  (bind _rtcengine_ref (Variables|Default|GetRtcEngine_Ref)
    (:then
      (bind _returnvalue (Class|AgoraRtcEngine|JoinChannel _rtcengine_ref "" channelId (Class|KismetStringLibrary|ToInt64(String) (Variables|/Game/Multiplayer/Blueprints/BP_GateGameInstance.BP_GateGameInstance_C|GetUserID (CallFunction|GetGateInstance))) (Utilities|Struct|MakeChannelMediaOptions "AGORA_NULL_VALUE" "AGORA_NULL_VALUE")))
      (return (== _returnvalue 0)))
    (:else)))

(fn LeaveVoiceChannel
  (bind _rtcengine_ref (Variables|Default|GetRtcEngine_Ref)
    (:then
      (Class|AgoraRtcEngine|LeaveChannel _rtcengine_ref (Utilities|Struct|MakeLeaveChannelOptions "AGORA_NULL_VALUE" "AGORA_NULL_VALUE" "AGORA_NULL_VALUE")))
    (:else)))

(fn SetDefaultAudioDevice
  (Variables|Default|GetAudioDeviceManager
    (:then
      (Utilities|FlowControl|Sequence
        (:then_0
          (bind _returnvalue (Class|IAudioDeviceManager|EnumerateRecordingDevices (Variables|Default|GetAudioDeviceManager)))
          (LocalVariables|SetLocalRecordingDevices _returnvalue)
          (bind _returnvalue_2 (Class|IAudioDeviceCollection|GetCount (LocalVariables|GetLocalRecordingDevices)))
          (bind _index (Utilities|FlowControl|ForLoopwithBreak 0 _returnvalue_2 :!label _label)
            (:LoopBody
              (bind (_devicename _deviceid) (Class|IAudioDeviceCollection|GetDevice (LocalVariables|GetLocalRecordingDevices) _index))
              (if (Utilities|String|Contains _devicename "Oculus Virtual Audio Device")
                (Variables|Default|SetMic_DeviceId _deviceid)
                (Class|IAudioDeviceManager|SetRecordingDevice (Variables|Default|GetAudioDeviceManager) (Variables|Default|GetMic_DeviceId))
                (goto _label Break)))))
        (:then_1
          (bind _returnvalue_3 (Class|IAudioDeviceManager|EnumeratePlaybackDevices (Variables|Default|GetAudioDeviceManager)))
          (LocalVariables|SetLocalPlaybackDevices _returnvalue_3)
          (bind _returnvalue_4 (Class|IAudioDeviceCollection|GetCount (LocalVariables|GetLocalPlaybackDevices)))
          (bind _index_2 (Utilities|FlowControl|ForLoopwithBreak 0 _returnvalue_4 :!label _label_2)
            (:LoopBody
              (bind (_devicename_2 _deviceid_2) (Class|IAudioDeviceCollection|GetDevice (LocalVariables|GetLocalPlaybackDevices) _index_2))
              (if (Utilities|String|Contains _devicename_2 "Oculus Virtual Audio Device")
                (Variables|Default|SetSpeaker_DeviceId _deviceid_2)
                (Class|IAudioDeviceManager|SetPlaybackDevice (Variables|Default|GetAudioDeviceManager) (Variables|Default|GetSpeaker_DeviceId))
                (goto _label_2 Break)))))))
    (:else)))

(fn UpdateSelfLocation
  (bind _localspatial (Variables|Default|GetLocalSpatial)
    (:then
      (bind _asbp_gate_character_vr (Utilities|Casting|CastToBP_GateCharacter_VR (Pawn|GetControlledPawn (Game|GetPlayerController 0))))
      (Class|ILocalSpatialAudioEngine|UpdateSelfPosition _localspatial (Transformation|GetWorldLocation (Variables|/Game/Multiplayer/Characters/FBIK/BP_GateCharacter_VR.BP_GateCharacter_VR_C|GetCamera _asbp_gate_character_vr)) (Math|Vector|GetForwardVector (Variables|/Game/Multiplayer/Characters/FBIK/BP_GateCharacter_VR.BP_GateCharacter_VR_C|GetCamera _asbp_gate_character_vr)) (Math|Vector|GetRightVector (Variables|/Game/Multiplayer/Characters/FBIK/BP_GateCharacter_VR.BP_GateCharacter_VR_C|GetCamera _asbp_gate_character_vr)) (Math|Vector|GetUpVector (Variables|/Game/Multiplayer/Characters/FBIK/BP_GateCharacter_VR.BP_GateCharacter_VR_C|GetCamera _asbp_gate_character_vr))))
    (:else)))

(fn UpdateRemoteLocation
  (params (RemotePlayerPosition :type Vector) (RemotePlayerForward :type Vector) (RemotePlayerUid :type String))
  (Variables|Default|GetLocalSpatial
    (:then
      (|SetBy-RefVar (stale _posinfo) (Utilities|Struct|MakeRemoteVoicePositionInfo RemotePlayerPosition RemotePlayerForward))
      (bind _posinfo (Class|ILocalSpatialAudioEngine|UpdateRemotePosition (Variables|Default|GetLocalSpatial) (Class|KismetStringLibrary|ToInt64(String) RemotePlayerUid))))
    (:else)))

(fn MuteVoice
  (params (mute :type Boolean))
  (bind _rtcengine_ref (Variables|Default|GetRtcEngine_Ref)
    (:then
      (Variables|Default|SetIsMicMute mute)
      (bind _returnvalue (Class|AgoraRtcEngine|MuteLocalAudioStream _rtcengine_ref mute))
      (return (== _returnvalue 0)))
    (:else)))

(fn EnableVolumeIndication
  (params (BindEvent :type Delegate%20%28by%20ref%29))
  (Utilities|FlowControl|Sequence
    (:then_0
      (bind _rtcengine_eventhandle (Variables|Default|GetRtcEngine_EventHandle)
        (:then
          (EventDispatchers|BindEventtoOnAudioVolumeIndication _rtcengine_eventhandle BindEvent))
        (:else)))
    (:then_1
      (bind _rtcengine_ref (Variables|Default|GetRtcEngine_Ref)
        (:then
          (Class|AgoraRtcEngine|EnableAudioVolumeIndication _rtcengine_ref 50 3 true))
        (:else)))))

(fn DisableVolumeIndication
  (Utilities|FlowControl|Sequence
    (:then_0
      (bind _rtcengine_eventhandle (Variables|Default|GetRtcEngine_EventHandle)
        (:then
          (EventDispatchers|UnbindallEventsfromOnAudioVolumeIndication _rtcengine_eventhandle))
        (:else)))))

(fn ToggleVoiceEcho
  (params (Enable :type Boolean))
  (bind _rtcengine_ref (Variables|Default|GetRtcEngine_Ref)
    (:then
      (Class|AgoraRtcEngine|SetAudioEffectPreset _rtcengine_ref (select Enable (Utilities|Struct|MakeENUMWRAP_AUDIO_EFFECT_PRESET "ROOM_ACOUSTICS_VOCAL_CONCERT") (Utilities|Struct|MakeENUMWRAP_AUDIO_EFFECT_PRESET "AUDIO_EFFECT_OFF"))))
    (:else)))