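; Multiplayer VR player state that shares each user's personal data and talking indicator through a name-tag actor attached to the character's body.
; Remote instances send game-instance data to the server on BeginPlay; its OnRep starts a looping timer that retries until the tag exists, then applies data and visibility.
; A bindable volume-indication callback derives talking state from local speaker volume and mic mute, relaying it via server and multicast to the tag.
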(event Custom|SendUserData_Server
  (params (State :type F%20Player%20Name%20Tag%20Structure))
  (Variables|NameTag|SetPersonalState State))

(event EventBeginPlay
  (if (not (Class|KismetSystemLibrary|IsStandalone))
    (Networking|SwitchHasAuthority
      (:Remote
        (Utilities|IsValid (Game|GetPlayerController)
          (:Is%20Valid
            (NameTag|SendUserData)))))))

(event Custom|SetUserTaking_Server
  (params (IsTalking :type Boolean))
  (CallFunction|SetUserTakingMulti IsTalking))

(event Custom|SetUserTaking_Multi
  (params (IsTaking :type Boolean))
  (Variables|NameTag|SetIsTalking IsTaking)
  (bind _personalstateui (Variables|NameTag|GetPersonalStateUI)
    (:then
      (Default|SetUserTalking _personalstateui (Variables|NameTag|GetIsTalking)))
    (:else)))

(fn ConstructionScript)

(fn SpawnPersonalStateUI
  (params (Owner :type Player%20Controller%20Object%20Reference))
  (Variables|NameTag|GetPersonalStateUI
    (:then
      _)
    (:else
      (bind _returnvalue (Game|SpawnActorfromClass "/Game/XHUD/Profile/BM_PersonalState.BM_PersonalState_C" (Math|Transform|MakeTransform "0, 0, 0" "0, 0, 0" "1.000000,1.000000,1.000000") "AlwaysSpawn" "OverrideRootScale" Owner 0))
      (Variables|NameTag|SetPersonalStateUI _returnvalue)))
  (bind _asbp_gate_character_vr (Utilities|Casting|CastToBP_GateCharacter_VR (Pawn|GetControlledPawn Owner)))
  (Default|SetAttachto (Variables|NameTag|GetPersonalStateUI) (Variables|/Game/Multiplayer/Characters/BP_GateCharacter_Base.BP_GateCharacter_Base_C|GetBody _asbp_gate_character_vr)))

(fn OnRepPersonalState
  (bind _returnvalue (Utilities|Time|SetTimerbyEvent (EventDispatchers|CreateEvent :!event UpdateState) 0.1 true))
  (Variables|NameTag|SetUpdateState_Timer _returnvalue))

(fn SendUserData
  (CallFunction|SendUserDataServer (Variables|/Game/Multiplayer/Blueprints/BP_GateGameInstance.BP_GateGameInstance_C|GetPersonalState (CallFunction|GetGateInstance))))

(fn UpdateState
  (bind _personalstateui (Variables|NameTag|GetPersonalStateUI)
    (:then
      (Default|UpdateState _personalstateui (Variables|NameTag|GetPersonalState))
      (Default|SetVisible _personalstateui (Variables|/Game/Multiplayer/Blueprints/BP_GateGameInstance.BP_GateGameInstance_C|GetIsNameTagOn (CallFunction|GetGateInstance)))
      (Utilities|Time|ClearandInvalidateTimerbyHandle (Variables|NameTag|GetUpdateState_Timer)))
    (:else)))

(fn SetUserTalking
  (params (IsTaking :type Boolean))
  (if (Pawn|IsLocalController (Game|GetPlayerController 0))
    (CallFunction|SetUserTakingServer IsTaking)))

(fn VolumeIndication
  (params (speakers :type Array%20of%20Audio%20Volume%20Info%20Structures) (totalVolume :type Integer))
  ;[1 1 1] Check LocalUser
  (if (== (Utilities|Array|Length speakers) 1)
    ;[1 1 1] CheckUsertaking
    (NameTag|SetUserTalking (or (== (.volume (Utilities|Struct|BreakAudioVolumeInfo (Utilities|Array|Get(acopy) speakers))) 0) (Variables|/Game/Multiplayer/Blueprints/BP_GateGameInstance.BP_GateGameInstance_C|GetIsMicMute (CallFunction|GetGateInstance))))
    (return)))

(fn SetBindVolumeIndication
  (params (IsBind :type Boolean))
  (if IsBind
    (Default|EnableVolumeIndication (CallFunction|GetGateInstance) (EventDispatchers|CreateEvent :!event VolumeIndication))
    (else
      (Default|DisableVolumeIndication (CallFunction|GetGateInstance)))))