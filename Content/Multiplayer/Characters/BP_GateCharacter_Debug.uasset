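; Desktop debug variant of the multiplayer VR Gate character that disables the HMD, removes face tracking and runs on mouse and keyboard.
; Each tick it pins both motion controllers in front of the camera, nudges the camera from arrow-key offsets and runs the teleport trace.
; Mouse and keys drive look, movement, crouch, teleport, calibration, plus grab and trigger for the hand chosen by Space.
; HUD key bindings are disabled.
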(event EventBeginPlay
  ;[1 1 1] Begin & Tick
  (|CallParentFunction)
  (Class|HeadMountedDisplayFunctionLibrary|EnableHMD false)
  (Components|DestroyComponent (Variables|Default|GetGateXRFaceTracking)))

(event EventTick
  (params (DeltaSeconds :type Float%20%28single-precision%29))
  ;[1 1 1] Begin & Tick
  (|CallParentFunction DeltaSeconds)
  (CallFunction|UpdateHandPose)
  (CallFunction|UpdateRelativeMovement)
  (CallFunction|TeleportTrace))

(event Input|AxisEvents|InputAxisLookUp
  (params (AxisValue :type Float%20%28single-precision%29))
  ;[1 1 1] LookUp
  (Transformation|AddRelativeRotation (Variables|Default|GetCamera) (Math|Rotator|MakeRotator 0.0 (* AxisValue -1.0) 0.0) false false))

(event Input|AxisEvents|InputAxisMoveForward/Backward
  (params (AxisValue :type Float%20%28single-precision%29))
  ;[1 1 1] Input Move & Trun
  (CallFunction|InputForward AxisValue))

(event Input|AxisEvents|InputAxisMoveRight/Left
  (params (AxisValue :type Float%20%28single-precision%29))
  ;[1 1 1] Input Move & Trun
  (CallFunction|InputRight AxisValue))

(event Input|AxisEvents|InputAxisTurnRight/LeftMouse
  (params (AxisValue :type Float%20%28single-precision%29))
  ;[1 1 1] Input Move & Trun
  (CallFunction|InputTurning AxisValue))

(event Input|MouseEvents|MouseWheelAxis
  (params (AxisValue :type Float%20%28single-precision%29))
  ;[1 1 1] Wheel - Relative Rotate Head
  (Transformation|AddRelativeRotation (Variables|Default|GetCamera) (Math|Rotator|MakeRotator 0.0 0.0 (* AxisValue (* (Utilities|Time|GetWorldDeltaSeconds) 1.8e+02))) false false))

(event Input|KeyboardEvents|DebugKeySpaceBar
  (params (Key :type Key%20Structure :default "None") (ActionValue :type Input%20Action%20Value%20Structure))
  ;[1 1 1] Space Bar - Swap Hand
  (:Pressed
    (bind _isa (Utilities|FlowControl|FlipFlop)
      (:A
        _)
      (:B
        _))
    (Variables|Default|SetIsLeft _isa)))

(event Input|KeyboardEvents|R
  (params (Key :type Key%20Structure :default "None"))
  ;[1 1 1] R - Calibration
  (:Pressed
    (CallFunction|Calibration)))

(event Input|MouseEvents|LeftMouseButton
  (params (Key :type Key%20Structure :default "None"))
  (bind _controller (CallFunction|GetGateController))
  (bind _isleft (Variables|Default|GetIsLeft))
  ;[1 1 1] Left Click - Trigger
  (:Pressed
    (Default|TriggerStart _controller _isleft))
  (:Released
    (Default|TriggerRelease _controller _isleft)))

(event Input|KeyboardEvents|G
  (params (Key :type Key%20Structure :default "None"))
  ;[1 1 1] HUD
  (:Pressed
    (Default|CancelFunctionsAll (CallFunction|GetGateController))))

(event Input|KeyboardEvents|X
  (params (Key :type Key%20Structure :default "None"))
  (bind _controller (CallFunction|GetGateController))
  ;[1 1 1] HUD
  (:Pressed
    (Default|InputNextSectorControllerHUD _controller 1.0)
    (Default|InputNextSectorControllerHUD _controller 0.0)))

(event Input|KeyboardEvents|Z
  (params (Key :type Key%20Structure :default "None"))
  (bind _controller (CallFunction|GetGateController))
  ;[1 1 1] HUD
  (:Pressed
    (Default|InputNextSectorControllerHUD _controller -1.0)
    (Default|InputNextSectorControllerHUD _controller 0.0)))

(event Input|KeyboardEvents|V
  (params (Key :type Key%20Structure :default "None"))
  ;[1 1 1] HUD
  (:Pressed
    (Default|InputSelectHUD (CallFunction|GetGateController))))

(event Input|MouseEvents|RightMouseButton
  (params (Key :type Key%20Structure :default "None"))
  (bind _isleft (Variables|Default|GetIsLeft))
  ;[1 1 1] Right Click - Grab
  (:Pressed
    (bind _vrik (Variables|Default|GetVRIK)
      (:then
        (Default|TryGrabServer _vrik _isleft))
      (:else)))
  (:Released
    (bind _vrik_2 (Variables|Default|GetVRIK)
      (:then
        (Default|TryReleaseServer _vrik_2 _isleft))
      (:else))))

(event Input|KeyboardEvents|C
  (params (Key :type Key%20Structure :default "None"))
  (bind _camera (Variables|Default|GetCamera))
  (bind _relativelocation (Variables|/Script/Engine.SceneComponent|GetRelativeLocation _camera))
  ;[1 1 1] C - Crouch
  (:Pressed
    (bind _isa (Utilities|FlowControl|FlipFlop)
      (:A
        _)
      (:B
        _))
    (Transformation|SetRelativeLocation (Variables|Default|GetCamera) (Math|Vector|MakeVector (.x _relativelocation) (.y _relativelocation) (Math|Float|SelectFloat 1.1e+02 157.0 _isa)) false false)))

(event Input|KeyboardEvents|Up
  (params (Key :type Key%20Structure :default "None"))
  ;[1 1 1] Arrow Keys - Relative Movement
  (:Pressed
    (Variables|Default|SetRelativeMovementAxisY (+ (Variables|Default|GetRelativeMovementAxisY) 1.0)))
  (:Released
    (Variables|Default|SetRelativeMovementAxisY (+ (Variables|Default|GetRelativeMovementAxisY) -1.0))))

(event Input|KeyboardEvents|Down
  (params (Key :type Key%20Structure :default "None"))
  ;[1 1 1] Arrow Keys - Relative Movement
  (:Pressed
    (Variables|Default|SetRelativeMovementAxisY (+ (Variables|Default|GetRelativeMovementAxisY) -1.0)))
  (:Released
    (Variables|Default|SetRelativeMovementAxisY (+ (Variables|Default|GetRelativeMovementAxisY) 1.0))))

(event Input|KeyboardEvents|Left
  (params (Key :type Key%20Structure :default "None"))
  ;[1 1 1] Arrow Keys - Relative Movement
  (:Pressed
    (Variables|Default|SetRelativeMovementAxisX (+ (Variables|Default|GetRelativeMovementAxisX) -1.0)))
  (:Released
    (Variables|Default|SetRelativeMovementAxisX (+ (Variables|Default|GetRelativeMovementAxisX) 1.0))))

(event Input|KeyboardEvents|Right
  (params (Key :type Key%20Structure :default "None"))
  ;[1 1 1] Arrow Keys - Relative Movement
  (:Pressed
    (Variables|Default|SetRelativeMovementAxisX (+ (Variables|Default|GetRelativeMovementAxisX) 1.0)))
  (:Released
    (Variables|Default|SetRelativeMovementAxisX (+ (Variables|Default|GetRelativeMovementAxisX) -1.0))))

(event Input|MouseEvents|MiddleMouseButton
  (params (Key :type Key%20Structure :default "None"))
  ;[1 1 1] Wheel Click - Teleport
  (:Pressed
    (CallFunction|StartTeleportTrace))
  (:Released
    (CallFunction|EndTeleportTrace)))

(event Input|KeyboardEvents|F
  (params (Key :type Key%20Structure :default "None"))
  ;[1 1 1] HUD
  (:Pressed
    (Default|ToggleSlotMenuHUD (CallFunction|GetGateController) true)))

(fn ConstructionScript
  (|CallParentFunction))

(fn UpdateHandPose
  (bind _camera (Variables|Default|GetCamera))
  (bind _camera_2 (Variables|Default|GetCamera))
  (bind _returnvalue (Transformation|GetWorldTransform _camera))
  (bind _returnvalue_2 (Transformation|GetWorldTransform _camera_2))
  (bind _returnvalue_3 (Math|Vector|GetRightVector (.rotation _returnvalue_2)))
  (bind _returnvalue_4 (Math|Vector|GetUpVector (.rotation _returnvalue_2)))
  (bind _returnvalue_5 (Math|Vector|GetForwardVector (.rotation _returnvalue_2)))
  (bind _returnvalue_6 (Math|Vector|GetForwardVector (.rotation _returnvalue)))
  (bind _returnvalue_7 (Math|Vector|GetRightVector (.rotation _returnvalue)))
  (bind _returnvalue_8 (Math|Vector|GetUpVector (.rotation _returnvalue)))
  (bind _returnvalue_9 (* _returnvalue_6 5e+01))
  (bind _returnvalue_10 (* _returnvalue_4 -1e+01))
  (bind _returnvalue_11 (* _returnvalue_3 -5.0))
  (bind _returnvalue_12 (* _returnvalue_5 5e+01))
  (bind _returnvalue_13 (* _returnvalue_7 5.0))
  (bind _returnvalue_14 (* _returnvalue_8 -1e+01))
  (bind _returnvalue_15 (+ (.location _returnvalue) _returnvalue_9 _returnvalue_13 _returnvalue_14))
  (bind _returnvalue_16 (+ (.location _returnvalue_2) _returnvalue_12 _returnvalue_11 _returnvalue_10))
  (Utilities|FlowControl|Sequence
    (:then_0
      (Transformation|SetWorldLocationAndRotation (Variables|Default|GetMotionControllerR) _returnvalue_15 (Math|Rotator|FindLookatRotation _returnvalue_15 (+ (.location _returnvalue) (* (Math|Vector|GetForwardVector (.rotation _returnvalue)) 1e+03))) false false)
      (Transformation|AddRelativeRotation (Variables|Default|GetMotionControllerR) (Math|Rotator|MakeRotator 0.0 (* (.pitch (Variables|/Script/Engine.SceneComponent|GetRelativeRotation (Variables|Default|GetControllerOffsetRootR))) -1) 0.0) false false))
    (:then_1
      (Transformation|SetWorldLocationAndRotation (Variables|Default|GetMotionControllerL) _returnvalue_16 (Math|Rotator|FindLookatRotation _returnvalue_16 (+ (.location _returnvalue_2) (* (Math|Vector|GetForwardVector (.rotation _returnvalue_2)) 1e+03))) false false)
      (Transformation|AddRelativeRotation (Variables|Default|GetMotionControllerL) (Math|Rotator|MakeRotator 0.0 (* (.pitch (Variables|/Script/Engine.SceneComponent|GetRelativeRotation (Variables|Default|GetControllerOffsetRootL))) -1) 0.0) false false))))

(fn UpdateFaceExpression)

(fn SendFaceExpression)

(fn InitFaceTracking)

(fn UpdateRelativeMovement
  (bind _camera (Variables|Default|GetCamera))
  (Transformation|AddWorldOffset (Variables|Default|GetCamera) (+ (* (Math|Vector|ProjectVectorontoPlane (Math|Vector|GetForwardVector _camera) "0.000000,0.000000,1.000000") (Variables|Default|GetRelativeMovementAxisY)) (* (Math|Vector|ProjectVectorontoPlane (Math|Vector|GetRightVector _camera) "0.000000,0.000000,1.000000") (Variables|Default|GetRelativeMovementAxisX))) false false))