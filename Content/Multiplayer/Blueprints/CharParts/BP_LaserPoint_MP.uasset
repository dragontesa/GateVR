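; Multiplayer VR laser pointer attached to a motion controller for targeting actors, operating widgets and carrying objects at range.
; Each tick a smoothed line trace sends interaction start/end messages and places the spline laser, gaze dot and widget interaction.
; Actors implementing the attach interface can follow a detached, interpolated attach point at adjustable distance.
; Pinch mode swaps the laser for a pinch mesh; player pawn destruction releases and destroys the pointer.
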(event Custom|DestroyLaser
  (params (DestroyedActor :type Actor%20Object%20Reference))
  ;[1 1 1] DestroyActor
  (if (not (Game|IsActorBeingDestroyed))
    (Attachment|DetachActor)
    (Actor|DestroyActor)))

(event Custom|DestroyBind
  ;[1 1 1] DestroyActor
  (Game|BindEventtoOnDestroyed (Game|Player|GetPlayerPawn 0) (delegate Custom|DestroyLaser)))

(event EventBeginPlay
  ;[1 1 1] BeginPlay
  (Construct|TogglePinchMode)
  (Construct|AttachActortoOwner)
  (CallFunction|DestroyBind)
  (CallFunction|SetLaserMaterial)
  (Variables|LineTrace|SetTraceRotation (Transformation|GetActorRotation))
  (Transformation|DetachFromComponent (Variables|Default|GetAttachPoint) "KeepWorld" "KeepWorld" "KeepWorld" true))

(event EventDestroyed
  ;[1 1 1] DestroyActor
  (bind _hit_actor (Variables|LineTrace|GetHit%20Actor)
    (:then
      (Class|BPInterfaceInteractionActor|InteractionEnd(Message) _hit_actor))
    (:else)))

(event EventTick
  (params (DeltaSeconds :type Float%20%28single-precision%29))
  ;[1 1 1] Tick
  (Update|UpdateLaser))

(fn ConstructionScript
  (Construct|UpdateLaserThickness)
  (Construct|InitLaserMaterialInstance)
  (Variables|/Script/UMG.WidgetInteractionComponent|SetInteractionDistance (Variables|Default|GetWidgetInteraction) (Variables|Setup|GetInteraction%20Distance)))

(fn InitLaserMaterialInstance
  (bind _returnvalue (Rendering|Material|CreateDynamicMaterialInstance (Variables|Default|GetLaser) 0 0 "None" :!class /Script/Engine.PrimitiveComponent))
  (Variables|Construction|SetMI_Laser _returnvalue))

(fn UpdateLaserThickness
  (SplineMesh|SetStartScale (Variables|Default|GetLaser) "(X=0.300000,Y=0.300000)" false :!class /Script/Engine.SplineMeshComponent)
  (SplineMesh|SetEndScale (Variables|Default|GetLaser) "(X=0.010000,Y=0.010000)" true :!class /Script/Engine.SplineMeshComponent))

(fn UpdateLaser
  (Variables|LineTrace|SetTraceRotation (Math|Interpolation|RInterpTo (Variables|LineTrace|GetTraceRotation) (Transformation|GetActorRotation) (Utilities|Time|GetWorldDeltaSeconds) 1e+01))
  (Utilities|FlowControl|Sequence
    (:then_0
      (if (Variables|Attachment|GetIsAttachActor)
        (Update|UpdateLaserforAttached)
        (elif (Update|TraceLaserHit)
          (Update|UpdateLaserforObject)
          (else
            (Update|UpdateLaserforNothing)))))
    (:then_1
      (Update|SetEndPoint))))

(fn IsOverlapWidget
  (bind _widgetinteraction (Variables|Default|GetWidgetInteraction))
  (return (or (Class|WidgetInteractionComponent|IsOverInteractableWidget _widgetinteraction) (Class|WidgetInteractionComponent|IsOverFocusableWidget _widgetinteraction))))

(fn TraceLaserHit
  (bind _returnvalue (Transformation|GetActorLocation))
  (Utilities|FlowControl|Sequence
    (:then_0
      (bind _owningmotioncontroller (Variables|Default|GetOwningMotionController)
        (:then
          (LocalVariables|SetActorsToIngnore (Utilities|Array|MakeArray (Components|GetOwner _owningmotioncontroller))))
        (:else)))
    (:then_1
      (bind (_outhit _returnvalue_2) (Collision|LineTraceByChannel _returnvalue (+ _returnvalue (* (Math|Vector|GetForwardVector (Variables|LineTrace|GetTraceRotation)) (Variables|Setup|GetInteraction%20Distance))) "TraceTypeQuery7" false (LocalVariables|GetActorsToIngnore) "None" true "(R=0.000000,G=0.000000,B=1.000000,A=1.000000)"))
      (Variables|LineTrace|SetLastHitResult _outhit)
      (return _returnvalue_2))))

(fn UpdateLaserforObject
  (bind _lasthitresult (Variables|LineTrace|GetLastHitResult))
  (bind _owningmotioncontroller (Variables|Default|GetOwningMotionController))
  (bind (_bblockinghit _binitialoverlap _time _distance _location _impactpoint _normal _impactnormal _physmat _hitactor) (Collision|BreakHitResult _lasthitresult))
  (Utilities|FlowControl|Sequence
    (:then_0
      (bind _hit_actor (Variables|LineTrace|GetHit%20Actor)
        (:then
          (if (!= _hit_actor _hitactor)
            (Class|BPInterfaceInteractionActor|InteractionEnd(Message) _hit_actor)))
        (:else)))
    (:then_1
      (Variables|LineTrace|SetHit%20Actor _hitactor)
      (Variables|LineTrace|SetImpact%20Point _impactpoint)
      (Variables|LineTrace|SetImpact%20Normal _impactnormal)
      (Variables|LineTrace|SetImpact%20Distance _distance)
      (Class|BPInterfaceInteractionActor|InteractionStart(Message) (Variables|LineTrace|GetHit%20Actor) _owningmotioncontroller (Components|GetOwner _owningmotioncontroller)))
    (:then_2
      (Rendering|SetVisibility (Variables|Default|GetGazePoint) true false)
      (Variables|PinchMode|SetPinchLength (Math|Float|MapRangeClamped (Variables|LineTrace|GetImpact%20Distance) 0.0 2e+02 0.0 1.0))
      (bind _mi_laser (Variables|Construction|GetMI_Laser)
        (:then
          (Rendering|Material|SetScalarParameterValue _mi_laser "opacity" 3e+01 :!class /Script/Engine.MaterialInstanceDynamic))
        (:else)))))

(fn UpdateLaserforNothing
  (bind _returnvalue (Transformation|GetActorForwardVector))
  (Utilities|FlowControl|Sequence
    (:then_0
      (bind _hit_actor (Variables|LineTrace|GetHit%20Actor)
        (:then
          (Class|BPInterfaceInteractionActor|InteractionEnd(Message) _hit_actor)
          (Variables|LineTrace|SetHit%20Actor 0))
        (:else)))
    (:then_1
      (Rendering|SetVisibility (Variables|Default|GetGazePoint) false false)
      (Variables|LineTrace|SetImpact%20Distance (Variables|Setup|GetNoHitLaserLength))
      (Variables|LineTrace|SetImpact%20Normal _returnvalue)
      (Variables|LineTrace|SetImpact%20Point (+ (Transformation|GetActorLocation) (* _returnvalue (Variables|Setup|GetNoHitLaserLength))))
      (Variables|PinchMode|SetPinchLength 0.0)
      (bind _mi_laser (Variables|Construction|GetMI_Laser)
        (:then
          (Rendering|Material|SetScalarParameterValue _mi_laser "opacity" 15.0 :!class /Script/Engine.MaterialInstanceDynamic))
        (:else)))))

(fn UpdateLaserforAttached
  (bind _tracerotation (Variables|LineTrace|GetTraceRotation))
  (bind _returnvalue (Math|Vector|GetForwardVector _tracerotation))
  (Variables|LineTrace|SetImpact%20Normal (* _returnvalue -1))
  (Variables|LineTrace|SetImpact%20Point (+ (Transformation|GetActorLocation) (* _returnvalue (Variables|LineTrace|GetImpact%20Distance))))
  (Rendering|SetVisibility (Variables|Default|GetGazePoint) false false))

(fn SetEndPoint
  (bind _returnvalue (Utilities|Time|GetWorldDeltaSeconds))
  (bind _impact_distance (Variables|LineTrace|GetImpact%20Distance))
  (bind _gazepoint (Variables|Default|GetGazePoint))
  (bind _gazescaledistance_min (LocalVariables|GetGazeScaleDistance_Min))
  (bind _attachpoint (Variables|Default|GetAttachPoint))
  (bind _interpspeed_attachment (LocalVariables|GetInterpSpeed_Attachment))
  (bind _interaction_distance (Variables|Setup|GetInteraction%20Distance))
  (bind _endpointsize_min (Variables|Setup|GetEndPointSize_Min))
  (bind _endpointsize_max (Variables|Setup|GetEndPointSize_Max))
  (bind _returnvalue_2 (Transformation|GetWorldTransform _gazepoint))
  (bind _returnvalue_3 (Transformation|GetWorldTransform _attachpoint))
  (bind _returnvalue_4 (Math|Float|MapRangeClamped _impact_distance _gazescaledistance_min _interaction_distance _endpointsize_min _endpointsize_max))
  (Utilities|FlowControl|Sequence
    (:then_0
      (Transformation|SetRelativeScale3D (Variables|Default|GetGazePoint) (Math|Vector|MakeVector (Variables|Setup|GetEndPointThickness) _returnvalue_4 _returnvalue_4))
      (Transformation|SetRelativeLocation (Variables|Default|GetGazePoint) (Math|Transform|InverseTransformLocation (Transformation|GetActorTransform) (+ (Variables|LineTrace|GetImpact%20Point) (* (Variables|LineTrace|GetImpact%20Normal) (Variables|Setup|GetEndPointHoverRate)))) false true)
      (if (not (Variables|Attachment|GetIsAttachActor))
        (Transformation|SetWorldRotation (Variables|Default|GetGazePoint) (Math|Rotator|MakeRotfromX (Variables|LineTrace|GetImpact%20Normal)) false false)))
    (:then_1
      (SplineMesh|SetEndPosition (Variables|Default|GetLaser) (Math|Transform|InverseTransformLocation (Transformation|GetActorTransform) (+ (Variables|LineTrace|GetImpact%20Point) (* (Variables|LineTrace|GetImpact%20Normal) (Variables|Setup|GetEndPointHoverRate)))) false)
      (SplineMesh|SetStartTangent (Variables|Default|GetLaser) (Math|Vector|MakeVector (Math|Float|Clamp(Float) (.x (Variables|/Script/Engine.SceneComponent|GetRelativeLocation (Variables|Default|GetGazePoint))) 0.0 (LocalVariables|GetTangent_Max)) 0.0 0.0) true :!class /Script/Engine.SplineMeshComponent))
    (:then_2
      (Transformation|SetWorldRotation (Variables|Default|GetWidgetInteraction) (Math|Rotator|FindLookatRotation (Transformation|GetActorLocation) (Variables|LineTrace|GetImpact%20Point)) false false))
    (:then_3
      (Transformation|SetWorldLocationAndRotation _attachpoint (Math|Interpolation|VInterpTo (.location _returnvalue_3) (.location _returnvalue_2) _returnvalue _interpspeed_attachment) (Math|Interpolation|RInterpTo (.rotation _returnvalue_3) (.rotation _returnvalue_2) _returnvalue _interpspeed_attachment) false false))))

(fn TriggerStart
  (Class|WidgetInteractionComponent|PressPointerKey (Variables|Default|GetWidgetInteraction) "LeftMouseButton"))

(fn TriggerRelease
  (Class|WidgetInteractionComponent|ReleasePointerKey (Variables|Default|GetWidgetInteraction) "LeftMouseButton"))

(fn UpdatePinchRate
  (params (PinchRate :type Float%20%28double-precision%29))
  (Variables|PinchMode|SetPinchRate PinchRate))

(fn AttachActortoOwner
  (bind _attachto (Variables|Default|GetAttachTo)
    (:then
      (Transformation|AttachComponentToComponent _attachto "None" "SnapToTarget" "SnapToTarget" "KeepWorld" false))
    (:else
      (Transformation|AttachComponentToComponent (Variables|Default|GetOwningMotionController) "None" "SnapToTarget" "SnapToTarget" "KeepWorld" false))))

(fn TogglePinchMode
  (Development|SetHiddeninGame (Variables|Default|GetLaser) (Variables|PinchMode|GetIsPinchMode) false)
  (Rendering|SetVisibility (Variables|Default|GetPinchMesh) (Variables|PinchMode|GetIsPinchMode) false))

(fn TryAttachHitActor
  (bind _gazepoint (Variables|Default|GetGazePoint))
  (bind _returnvalue (Transformation|GetWorldTransform _gazepoint))
  (bind _hit_actor (Variables|LineTrace|GetHit%20Actor)
    (:then
      (if (Utilities|DoesObjectImplementInterface _hit_actor "/Game/Multiplayer/Blueprints/CharParts/BP_Interface_AttachActor.BP_Interface_AttachActor_C")
        (Transformation|SetWorldLocationAndRotation (Variables|Default|GetAttachPoint) (.location _returnvalue) (.rotation _returnvalue) false true)
        (bind (_isattach _attachactor) (Class|BPInterfaceAttachActor|AttachActorComp(Message) (Variables|LineTrace|GetHit%20Actor) (Variables|Default|GetAttachPoint)))
        (if _isattach
          (Variables|Attachment|SetAttachedActor _attachactor)
          (Variables|Attachment|SetIsAttachActor true)
          (return true)
          (else
            (return false)))
        (else
          (return false))))
    (:else
      (return false))))

(fn DetachActor
  (Utilities|FlowControl|Sequence
    (:then_0
      (bind _attachedactor (Variables|Attachment|GetAttachedActor)
        (:then
          (Class|BPInterfaceAttachActor|DetachActor(Message) _attachedactor))
        (:else)))
    (:then_1
      (Variables|Attachment|SetAttachedActor 0)
      (Variables|Attachment|SetIsAttachActor false))))

(fn AddAttachedDistance
  (params (Value :type Float%20%28double-precision%29))
  (if (Variables|Attachment|GetIsAttachActor)
    (Variables|LineTrace|SetImpact%20Distance (+ (Variables|LineTrace|GetImpact%20Distance) (* Value 1.5)))))

(fn SetLaserMaterial
  (Variables|Default|GetMaterial_Laser
    (:then
      (Rendering|Material|SetMaterial (Variables|Default|GetPinchMesh) 0 (Variables|Default|GetMaterial_Laser)))
    (:else)))