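; Debug game mode for multiplayer that respawns a player with a given character set.
; RespawnPlayer destroys the controller's old character, then calls SpawnPawn.
; SpawnPawn casts the default pawn class to BP_GateCharacter_Base, spawns it at a random non-host spawn point with the character set passed in, possesses it and creates that player's personal state UI.
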(event EventRespawnPlayer
  (params (Controller :type Player%20Controller%20Object%20Reference) (Character :type Character%20Preset%20Class%20Reference) (IsHost :type Boolean))
  (CallFunction|DestroyOldCharacter Controller)
  (CallFunction|SpawnPawn Controller Character))

(fn ConstructionScript
  (|CallParentFunction))

(fn SpawnPawn
  (params (Controller :type Player%20Controller%20Object%20Reference) (CharacterSet :type Character%20Preset%20Class%20Reference))
  (bind _asbp_gate_character_base (Utilities|Casting|CastToBP_GateCharacter_BaseClass (Variables|Default|GetDefaultPawnClass)))
  (bind _returnvalue (Game|SpawnActorfromClass _asbp_gate_character_base (Transformation|GetActorTransform (CallFunction|GetRandomSpawnPoint Controller false)) "AdjustIfPossibleButAlwaysSpawn" "SelectDefaultAtRuntime" 0 CharacterSet 0))
  (Pawn|Possess Controller _returnvalue)
  (CallFunction|SpawnPersonalStateUI Controller))