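; Game instance for a multiplayer VR game, holding user, character, session and save-game state across level travel.
; It runs Agora voice chat with mute, effects, spatial positioning and channel switching by rejoining after leave, released on level change or shutdown.
; Host and player data start GameLift sessions, falling back to socket messages or fixed-IP travel.
; It also fades the camera on travel or quit and prints network errors.
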(event Custom|OpenLevel
  (params (Level :type Name))
  ;[1 1 1] OpenLevel With Camera Fade
  (Plugin_Agora|ReleaseVoice)
  (CameraFades|StartCameraFade :self (Game|GetPlayerCameraManager 0) :ToAlpha 1.0 :Duration 1.5 :bHoldWhenFinished true)
  (Default|CallOnStartOpenLevel)
  (Utilities|FlowControl|Delay 5.0)
  (Game|OpenLevel(byName) Level))

(event Custom|ExitGame
  ;[1 1 1] Exit Game
  (CameraFades|StartCameraFade :self (Game|GetPlayerCameraManager 0) :ToAlpha 1.0 :Duration 1.5 :bHoldWhenFinished true)
  (Utilities|FlowControl|Delay 2.0)
  (Game|QuitGame (Game|GetPlayerController 0) "Quit" false))

(event EventShutdown
  ;[1 1 1] Shut Down
  (Plugin_Agora|ReleaseVoice))

(event EventHandleTravelError
  (params (FailureType :type ETravelFailure%20Enum :default "NoLevel"))
  ;[1 1 1] Handle Travel Errors
  (Debug|DisplayErrorMessage (Debug|TravelErrortoString FailureType)))

(event EventHandleNetworkError
  (params (FailureType :type ENetworkFailure%20Enum :default "NetDriverAlreadyExists") (bIsServer :type Boolean))
  ;[1 1 1] Handle Network Errors
  (Debug|DisplayErrorMessage (Debug|NetErrortoString FailureType)))

(event Custom|RequestAgoraReconnect
  (params (Channel :type String))
  (Variables|Plugin_Agora|SetReConnectVoiceChannelName Channel)
  (EventDispatchers|BindEventtoOnLeaveChannel (Variables|Plugin_Agora|GetRtcEngine_EventHandle) (delegate Custom|AgoraReconnecting))
  (Plugin_Agora|LeaveVoiceChannel))

(event Custom|AgoraReconnecting
  (params (stats :type Rtc%20Stats%20Structure%20%28by%20ref%29))
  (EventDispatchers|UnbindEventfromOnLeaveChannel (Variables|Plugin_Agora|GetRtcEngine_EventHandle) (delegate Custom|AgoraReconnecting))
  (Plugin_Agora|JoinVoiceChannel (Variables|Plugin_Agora|GetReConnectVoiceChannelName))
  (Variables|Plugin_Agora|SetReConnectVoiceChannelName ""))

(fn NetErrortoString
  (params (FailureType :type ENetworkFailure%20Enum :default "NetDriverAlreadyExists"))
  (return (Utilities|String|Append "Error " (Utilities|String|EnumtoString FailureType))))

(fn TravelErrortoString
  (params (FailureType :type ETravelFailure%20Enum :default "NoLevel"))
  (return (Utilities|String|Append "Error " (Utilities|String|EnumtoString FailureType))))

(fn DisplayErrorMessage
  (params (Message :type String))
  (Development|PrintString Message))

(fn DebugPrintMicSampling
  (params (data :type Array%20of%20Bytes))
  (if (Utilities|Array|IsNotEmpty data)
    (bind _output_get (LocalVariables|Setsamples data))
    (Development|PrintString (Utilities|String|Append "bp received data from mic " (Utilities|String|ToString(Integer) (Utilities|Array|Length _output_get))))))

(fn CheckSaveGame
  (bind _returnvalue (SaveGame|DoesSaveGameExist "PlayerSettingsSave"))
  (if _returnvalue
    (Save|LoadGame)
    (Save|SaveGame)
    (else
      (UserInfo|SetCharactertoRandom)
      (Save|SaveGame))))

(fn SaveGame
  (Variables|Save|GetPlayerSaveGameRef
    (:then
      _)
    (:else
      (bind _returnvalue (SaveGame|CreateSaveGameObject "/Game/Multiplayer/Blueprints/BP_PlayerSaveGameMP.BP_PlayerSaveGameMP_C"))
      (Variables|Save|SetPlayerSaveGameRef _returnvalue)))
  (Variables|/Game/Multiplayer/Blueprints/BP_PlayerSaveGameMP.BP_PlayerSaveGameMP_C|SetS_PlayerInfo (Variables|Save|GetPlayerSaveGameRef) (Variables|UserInfo|GetPlayerSettings))
  (bind _returnvalue_2 (SaveGame|SaveGametoSlot (Variables|Save|GetPlayerSaveGameRef) "PlayerSettingsSave"))
  (return _returnvalue_2))

(fn LoadGame
  (bind _returnvalue (SaveGame|DoesSaveGameExist "PlayerSettingsSave"))
  (if _returnvalue
    (bind _returnvalue_2 (SaveGame|LoadGamefromSlot "PlayerSettingsSave"))
    (bind _asbp_player_save_game_mp (Utilities|Casting|CastToBP_PlayerSaveGameMP _returnvalue_2)
      (:then
        (|SetBy-RefVar (Variables|UserInfo|GetPlayerSettings) (Variables|/Game/Multiplayer/Blueprints/BP_PlayerSaveGameMP.BP_PlayerSaveGameMP_C|GetS_PlayerInfo _asbp_player_save_game_mp))
        (return true))
      (:CastFailed
        (return false)))
    (else
      (return false))))

(fn SpawnGateGameLift
  (Variables|Plugin_GameLift|GetGateGameLiftRef
    (:then)
    (:else
      (bind _returnvalue (Game|SpawnActorfromClass "/Game/Multiplayer/GameLift/BP_HandleGateGameLift.BP_HandleGateGameLift_C" (Math|Transform|MakeTransform "0, 0, 0" "0, 0, 0" "1.000000,1.000000,1.000000") "Undefined" "OverrideRootScale" 0 0))
      (Variables|Plugin_GameLift|SetGateGameLiftRef _returnvalue)
      (return (Variables|Plugin_GameLift|GetGateGameLiftRef)))))

(fn InitVoice
  (bind _returnvalue (Game|GetPlayerController 0))
  (Variables|Plugin_Agora|GetRtcEngine_Ref
    (:then)
    (:else
      (bind _returnvalue_2 (Game|ConstructObjectfromClass _returnvalue "/Script/AgoraPlugin.IRtcEngineEventHandler"))
      (bind _output_get (Variables|Plugin_Agora|SetRtcEngine_EventHandle _returnvalue_2))
      (bind _returnvalue_3 (Game|ConstructObjectfromClass _returnvalue "/Script/AgoraPlugin.AgoraRtcEngine"))
      (bind _output_get_2 (Variables|Plugin_Agora|SetRtcEngine_Ref _returnvalue_3))
      (Class|AgoraRtcEngine|Initialize _output_get_2 (Utilities|Struct|MakeRtcEngineContext "13b44aa785094489a54fb06ee22d45c5" _output_get 0 "" "CHANNEL_PROFILE_COMMUNICATION" "AUDIO_SCENARIO_DEFAULT" false "HIGH"))
      (Class|AgoraRtcEngine|SetAudioProfile (Variables|Plugin_Agora|GetRtcEngine_Ref) "AUDIO_PROFILE_MUSIC_HIGH_QUALITY" "AUDIO_SCENARIO_DEFAULT")
      (Utilities|FlowControl|Sequence
        (:then_0
          (bind _returnvalue_4 (Class|AgoraRtcEngine|QueryInterface (Variables|Plugin_Agora|GetRtcEngine_Ref) "AGORA_IID_AUDIO_DEVICE_MANAGER"))
          (bind _asiaudio_device_manager (Utilities|Casting|CastToIAudioDeviceManager _returnvalue_4))
          (Variables|Plugin_Agora|SetAudioDeviceManager _asiaudio_device_manager))
        (:then_1
          (bind _returnvalue_5 (SaveGame|LoadGamefromSlot "Menu"))
          (bind _assave_menu (Utilities|Casting|CastToSave_Menu _returnvalue_5))
          (Plugin_Agora|MuteVoice (not (Variables|/Game/XHUD/SlotMenu/Save_Menu.Save_Menu_C|GetIsMic_On _assave_menu))))))))

(fn ReleaseVoice
  (bind _rtcengine_ref (Variables|Plugin_Agora|GetRtcEngine_Ref)
    (:then
      (Class|AgoraRtcEngine|LeaveChannel _rtcengine_ref (Utilities|Struct|MakeLeaveChannelOptions "AGORA_NULL_VALUE" "AGORA_NULL_VALUE" "AGORA_NULL_VALUE"))
      (bind _returnvalue (Class|AgoraRtcEngine|UnregisterEventHandler _rtcengine_ref (Variables|Plugin_Agora|GetRtcEngine_EventHandle)))
      (Development|PrintString (Utilities|String|Append "Rtc Handle Unregister : " (Utilities|String|ToString(Boolean) _returnvalue)) false)
      (Class|AgoraRtcEngine|Release _rtcengine_ref true)
      (Development|PrintString "Agora Release : True" false)
      (Variables|Plugin_Agora|SetRtcEngine_EventHandle 0)
      (Variables|Plugin_Agora|SetRtcEngine_Ref 0))
    (:else)))

(fn InitSpatialVoice
  (bind _returnvalue (Class|AgoraRtcEngine|QueryInterface (Variables|Plugin_Agora|GetRtcEngine_Ref) "AGORA_IID_LOCAL_SPATIAL_AUDIO"))
  (bind _asilocal_spatial_audio_engine (Utilities|Casting|CastToILocalSpatialAudioEngine _returnvalue))
  (bind _output_get (Variables|Plugin_Agora|SetLocalSpatial _asilocal_spatial_audio_engine))
  (|SetBy-RefVar (stale _config) (Utilities|Struct|MakeLocalSpatialAudioConfig (Variables|Plugin_Agora|GetRtcEngine_Ref)))
  (bind _config (Class|ILocalSpatialAudioEngine|Initialize _output_get))
  (Class|ILocalSpatialAudioEngine|SetAudioRecvRange (Variables|Plugin_Agora|GetLocalSpatial) 2e+04)
  (Class|ILocalSpatialAudioEngine|SetDistanceUnit (Variables|Plugin_Agora|GetLocalSpatial) 0.01))

(fn JoinVoiceChannel
  (params (channelId :type String))
  (bind _rtcengine_ref (Variables|Plugin_Agora|GetRtcEngine_Ref)
    (:then
      (bind _returnvalue (Class|AgoraRtcEngine|GetConnectionState _rtcengine_ref))
      (switch Utilities|FlowControl|Switch|SwitchonECONNECTION_STATE_TYPE _returnvalue
        (:CONNECTION_NULL
          (bind _returnvalue_2 (Class|AgoraRtcEngine|JoinChannel (Variables|Plugin_Agora|GetRtcEngine_Ref) "" channelId (Class|KismetStringLibrary|ToInt64(String) (Variables|UserInfo|GetUser_Code)) (Utilities|Struct|MakeChannelMediaOptions "AGORA_NULL_VALUE" "AGORA_NULL_VALUE") :!label _label))
          (Development|PrintString (Utilities|String|Append "Agora Join Channel Return Value : " (Utilities|String|ToString(Integer) _returnvalue_2)) false)
          (return (== _returnvalue_2 0)))
        (:CONNECTION_STATE_DISCONNECTED
          (goto _label))
        (:CONNECTION_STATE_CONNECTED
          (CallFunction|RequestAgoraReconnect channelId))))
    (:else)))

(fn LeaveVoiceChannel
  (bind _rtcengine_ref (Variables|Plugin_Agora|GetRtcEngine_Ref)
    (:then
      (Class|AgoraRtcEngine|LeaveChannel _rtcengine_ref (Utilities|Struct|MakeLeaveChannelOptions "AGORA_NULL_VALUE" "AGORA_NULL_VALUE" "AGORA_NULL_VALUE")))
    (:else)))

(fn OpenLobby
  (bind _returnvalue (Game|GetCurrentLevelName true))
  (LocalVariables|SetLocalCurrentLevelName _returnvalue)
  (if (not (Utilities|Array|ContainsItem (.list_levelname (Utilities|Struct|MakeFLobbyLevelList)) (LocalVariables|GetLocalCurrentLevelName)))
    (CallFunction|OpenLevel "LoadingLevel")))

(fn SetDefaultAudioDevice
  (Variables|Plugin_Agora|GetAudioDeviceManager
    (:then
      (Utilities|FlowControl|Sequence
        (:then_0
          (Class|IAudioDeviceManager|FollowSystemPlaybackDevice (Variables|Plugin_Agora|GetAudioDeviceManager) true))
        (:then_1
          (Class|IAudioDeviceManager|FollowSystemRecordingDevice (Variables|Plugin_Agora|GetAudioDeviceManager) true))))
    (:else)))

(fn SetDefaultAudioDeviceOld
  (Variables|Plugin_Agora|GetAudioDeviceManager
    (:then
      (Utilities|FlowControl|Sequence
        (:then_0
          (bind _returnvalue (Class|IAudioDeviceManager|EnumerateRecordingDevices (Variables|Plugin_Agora|GetAudioDeviceManager)))
          (LocalVariables|SetLocalRecordingDevices _returnvalue)
          (bind _returnvalue_2 (Class|IAudioDeviceCollection|GetCount (LocalVariables|GetLocalRecordingDevices)))
          (bind _index (Utilities|FlowControl|ForLoopwithBreak 0 _returnvalue_2 :!label _label)
            (:LoopBody
              (bind (_devicename _deviceid) (Class|IAudioDeviceCollection|GetDevice (LocalVariables|GetLocalRecordingDevices) _index))
              (if (Utilities|String|Contains _devicename "Oculus Virtual Audio Device")
                (Variables|Plugin_Agora|SetMic_DeviceId _deviceid)
                (Class|IAudioDeviceManager|SetRecordingDevice (Variables|Plugin_Agora|GetAudioDeviceManager) (Variables|Plugin_Agora|GetMic_DeviceId))
                (goto _label Break)))))
        (:then_1
          (bind _returnvalue_3 (Class|IAudioDeviceManager|EnumeratePlaybackDevices (Variables|Plugin_Agora|GetAudioDeviceManager)))
          (LocalVariables|SetLocalPlaybackDevices _returnvalue_3)
          (bind _returnvalue_4 (Class|IAudioDeviceCollection|GetCount (LocalVariables|GetLocalPlaybackDevices)))
          (bind _index_2 (Utilities|FlowControl|ForLoopwithBreak 0 _returnvalue_4 :!label _label_2)
            (:LoopBody
              (bind (_devicename_2 _deviceid_2) (Class|IAudioDeviceCollection|GetDevice (LocalVariables|GetLocalPlaybackDevices) _index_2))
              (if (Utilities|String|Contains _devicename_2 "Oculus Virtual Audio Device")
                (Variables|Plugin_Agora|SetSpeaker_DeviceId _deviceid_2)
                (Class|IAudioDeviceManager|SetPlaybackDevice (Variables|Plugin_Agora|GetAudioDeviceManager) (Variables|Plugin_Agora|GetSpeaker_DeviceId))
                (goto _label_2 Break)))))))
    (:else)))

(fn SetHostData
  (params (IsHost :type Boolean) (GameID :type String) (UserCount :type Integer) (GameType :type String) (MapName :type String) (InMatchingGame :type Boolean))
  (if IsHost
    (Variables|Platform|SetIsHost IsHost)
    (Variables|Platform|SetGame_ID GameID)
    (Variables|Platform|SetUserCount UserCount)
    (Variables|Platform|SetMapName MapName)
    (Variables|Matching|SetIsInMatchingGame InMatchingGame)
    (Variables|Matching|SetIsJoinMatchServer false)
    (if (CallFunction|IsGameLiftEnabled)
      (Plugin_GameLift|StartGameLiftSession)
      (elif (Variables|Matching|GetIsInMatchingGame)
        (bind _asbp_socket_io_random_chat (Utilities|Casting|CastToBP_SocketIO_RandomChat (Variables|/Game/Multiplayer/Blueprints/BP_GatePlayerController.BP_GatePlayerController_C|GetSocketIoRef (CallFunction|GetGateController))))
        (Default|Ue-matching-response-game-session _asbp_socket_io_random_chat "TEST")
        (else
          (Default|SendGameFleetID (Variables|/Game/Multiplayer/Blueprints/BP_GatePlayerController.BP_GatePlayerController_C|GetSocketIoRef (CallFunction|GetGateController)) "LocalDedicated"))))
    (else
      (Variables|Platform|SetIsHost false))))

(fn SetPlayerData
  (params (IsHost :type Boolean) (IsinGame :type Boolean) (UserCount :type Integer) (GameID :type String) (FleetID :type String) (GameType :type String) (IsTest :type Boolean))
  (Variables|Platform|SetIsHost IsHost)
  (Variables|Platform|SetIsInGame (LocalVariables|GetIsInGame))
  (Variables|Platform|SetUserCount UserCount)
  (Variables|Platform|SetGame_ID GameID)
  (Variables|Plugin_Agora|SetVoiceChannel GameID)
  (Variables|Plugin_GameLift|SetGamesession_ID FleetID)
  (Variables|Platform|SetGame_Type GameType)
  (Variables|Matching|SetIsJoinMatchServer false)
  (if (CallFunction|IsGameLiftEnabled)
    (Plugin_GameLift|StartGameLiftPlayer)
    (elif IsTest
      (CallFunction|OpenLevel "61.34.111.112:7778")
      (else
        (CallFunction|OpenLevel "61.34.111.112")))))

(fn StartGameLiftSession
  ;[0.1329 0.1912 0.2705] Touring GameLift Session
  (CallFunction|InitGameLift)
  (Plugin_GameLift|BindEventonCreateGameSession)
  (CallFunction|StartGameSession))

(fn StartGameLiftPlayer
  ;[0.1329 0.1912 0.2705] Start GameLift Player
  (CallFunction|InitGameLift)
  (CallFunction|StartPlayer))

(fn UpdateSelfLocation
  (bind _localspatial (Variables|Plugin_Agora|GetLocalSpatial)
    (:then
      (bind _asbp_gate_character_vr (Utilities|Casting|CastToBP_GateCharacter_VR (Pawn|GetControlledPawn (Game|GetPlayerController 0))))
      (Class|ILocalSpatialAudioEngine|UpdateSelfPosition _localspatial (Transformation|GetWorldLocation (Variables|/Game/Multiplayer/Characters/FBIK/BP_GateCharacter_VR.BP_GateCharacter_VR_C|GetCamera _asbp_gate_character_vr)) (Math|Vector|GetForwardVector (Variables|/Game/Multiplayer/Characters/FBIK/BP_GateCharacter_VR.BP_GateCharacter_VR_C|GetCamera _asbp_gate_character_vr)) (Math|Vector|GetRightVector (Variables|/Game/Multiplayer/Characters/FBIK/BP_GateCharacter_VR.BP_GateCharacter_VR_C|GetCamera _asbp_gate_character_vr)) (Math|Vector|GetUpVector (Variables|/Game/Multiplayer/Characters/FBIK/BP_GateCharacter_VR.BP_GateCharacter_VR_C|GetCamera _asbp_gate_character_vr))))
    (:else)))

(fn UpdateRemoteLocation
  (params (RemotePlayerPosition :type Vector) (RemotePlayerForward :type Vector) (RemotePlayerUid :type String))
  (Variables|Plugin_Agora|GetLocalSpatial
    (:then
      (|SetBy-RefVar (stale _posinfo) (Utilities|Struct|MakeRemoteVoicePositionInfo RemotePlayerPosition RemotePlayerForward))
      (bind _posinfo (Class|ILocalSpatialAudioEngine|UpdateRemotePosition (Variables|Plugin_Agora|GetLocalSpatial) (Class|KismetStringLibrary|ToInt64(String) RemotePlayerUid))))
    (:else)))

(fn NextLevel
  (bind _output_get (Variables|Platform|SetLobbyLevelNum (Math|Integer|%(Integer) (+ (Variables|Platform|GetLobbyLevelNum) 1) (Utilities|Array|Length (.list_levelname (Utilities|Struct|MakeFLobbyLevelList))))))
  (return _output_get))

(fn TryLogin
  (if (not (Variables|UserInfo|GetIsLogin))
    (Variables|UserInfo|SetIsLogin true)))

(fn LoginFailed
  (Variables|UserInfo|SetUser_Code ""))

(fn SpawnPixelStreamer
  (Game|SpawnActorfromClass "/Game/PixelStreaming/BP_PixelStreamingActor.BP_PixelStreamingActor_C" (Math|Transform|MakeTransform "0, 0, 0" "0, 0, 0" "1.000000,1.000000,1.000000") "Undefined" "OverrideRootScale" 0 0))

(fn FinishPixelStreaming
  (bind _returnvalue (Game|GetPlayerController 0))
  (bind _returnvalue_2 (Actor|GetComponentbyClass _returnvalue "/Game/PixelStreaming/BP_GatePixelStreamingInput.BP_GatePixelStreamingInput_C"))
  (Utilities|IsValid _returnvalue_2
    (:Is%20Valid
      (Components|DestroyComponent _returnvalue_2)
      (bind _pactor (CallFunction|GetPixelStreamingActor))
      (Utilities|IsValid _pactor
        (:Is%20Valid
          (Actor|DestroyActor _pactor))))))

(fn EnableVolumeIndication
  (params (BindEvent :type Delegate%20%28by%20ref%29))
  (Utilities|FlowControl|Sequence
    (:then_0
      (bind _rtcengine_eventhandle (Variables|Plugin_Agora|GetRtcEngine_EventHandle)
        (:then
          (EventDispatchers|BindEventtoOnAudioVolumeIndication _rtcengine_eventhandle BindEvent))
        (:else)))
    (:then_1
      (bind _rtcengine_ref (Variables|Plugin_Agora|GetRtcEngine_Ref)
        (:then
          (Class|AgoraRtcEngine|EnableAudioVolumeIndication _rtcengine_ref 50 3 true))
        (:else)))))

(fn DisableVolumeIndication
  (Utilities|FlowControl|Sequence
    (:then_0
      (bind _rtcengine_eventhandle (Variables|Plugin_Agora|GetRtcEngine_EventHandle)
        (:then
          (EventDispatchers|UnbindallEventsfromOnAudioVolumeIndication _rtcengine_eventhandle))
        (:else)))))

(fn JoinMatchServer
  (params (GameSessionID :type String))
  (Variables|Plugin_GameLift|SetGamesession_ID GameSessionID)
  (Variables|Platform|SetGame_ID "")
  (Variables|Matching|SetIsJoinMatchServer true)
  (if (CallFunction|IsGameLiftEnabled)
    (Plugin_GameLift|StartGameLiftPlayer)
    (else
      (CallFunction|OpenLevel "61.34.111.112"))))

(fn CreateGameLiftSession
  ;[0.1329 0.1912 0.2705] Create GameLift Session
  (CallFunction|InitGameLift)
  (CallFunction|StartGameSession))

(fn BindEventonCreateGameSession
  (Variables|Plugin_GameLift|GetGateGameLiftRef
    (:then
      (if (Variables|Matching|GetIsInMatchingGame)
        (bind _asbp_socket_io_random_chat (Utilities|Casting|CastToBP_SocketIO_RandomChat (Variables|/Game/Multiplayer/Blueprints/BP_GatePlayerController.BP_GatePlayerController_C|GetSocketIoRef (CallFunction|GetGateController))))
        (EventDispatchers|BindEventtoOnCreateGameSessionSuccess (Variables|Plugin_GameLift|GetGateGameLiftRef) (EventDispatchers|CreateEvent _asbp_socket_io_random_chat :!event Ue-matching-response-game-session))
        (else
          (EventDispatchers|BindEventtoOnCreateGameSessionSuccess (Variables|Plugin_GameLift|GetGateGameLiftRef) (EventDispatchers|CreateEvent (Variables|/Game/Multiplayer/Blueprints/BP_GatePlayerController.BP_GatePlayerController_C|GetSocketIoRef (CallFunction|GetGateController)) :!event SendGameFleetID)))))
    (:else)))

(fn MuteVoice
  (params (mute :type Boolean))
  (Variables|Plugin_Agora|SetIsMicMute mute)
  (bind _rtcengine_ref (Variables|Plugin_Agora|GetRtcEngine_Ref)
    (:then
      (bind _returnvalue (Class|AgoraRtcEngine|MuteLocalAudioStream _rtcengine_ref mute))
      (return (== _returnvalue 0)))
    (:else)))

(fn ToggleVoiceEcho
  (params (Enable :type Boolean))
  (bind _rtcengine_ref (Variables|Plugin_Agora|GetRtcEngine_Ref)
    (:then
      (Class|AgoraRtcEngine|SetAudioEffectPreset _rtcengine_ref (select Enable (Utilities|Struct|MakeENUMWRAP_AUDIO_EFFECT_PRESET "ROOM_ACOUSTICS_VOCAL_CONCERT") (Utilities|Struct|MakeENUMWRAP_AUDIO_EFFECT_PRESET "AUDIO_EFFECT_OFF"))))
    (:else)))

(fn SetVoiceEffect
  (params (Effect :type EENUMCUSTOM_VOICE_CONVERSION_PRESET%20Enum :default "VOICE_CONVERSION_OFF"))
  (bind _rtcengine_ref (Variables|Plugin_Agora|GetRtcEngine_Ref)
    (:then
      (Class|AgoraRtcEngine|SetVoiceConversionPreset _rtcengine_ref (Utilities|Struct|MakeENUMWRAP_VOICE_CONVERSION_PRESET Effect)))
    (:else)))

(fn SetUserIDCode
  (params (UserCode :type String) (UserId :type String))
  (Variables|UserInfo|SetUser_Code UserCode)
  (Variables|UserInfo|SetUser_Id UserId)
  (Variables|UserInfo|SetIsLogin true))

(fn SetUserInfo
  (params (CharacterCode :type String) (CurrentPartsInfo :type F%20Parts%20Info%20Structure))
  (Variables|UserInfo|SetCurrentCharacter%20Code CharacterCode)
  (Variables|UserInfo|SetCurrentPartsInfo CurrentPartsInfo))

(fn SetPartsInfo
  (params (CurrentPartsInfo :type F%20Parts%20Info%20Structure))
  (Variables|UserInfo|SetCurrentPartsInfo CurrentPartsInfo))

(fn SetCharacterGender
  (params (IsCurrentGenderMale :type Boolean))
  (Variables|UserInfo|SetIsMale IsCurrentGenderMale))

(fn SetCharacterCode
  (params (CurrentCharacterCode :type String))
  (Variables|UserInfo|SetCurrentCharacter%20Code CurrentCharacterCode))

(fn SetCharacterPreset
  (params (CurrentCharacterPreset :type Character%20Preset%20Class%20Reference))
  (Variables|UserInfo|SetCurrentCharacterPreset CurrentCharacterPreset))

(fn SetCharactertoRandom
  (bind _characters (Variables|CharacterPreset|GetCharacters))
  (Utilities|Struct|SetmembersinFPlayerInfo (Variables|UserInfo|GetPlayerSettings) (Utilities|Array|Get(acopy) _characters (Math|Random|RandomInteger (Utilities|Array|Length _characters)))))

(fn SetLanguage
  (params (Language :type ELanguage%20Enum :default "NewEnumerator2"))
  (Variables|UserInfo|SetCurrentLanguage Language))

(fn OnResponsePlayerState
  (params (PersonalState :type F%20Player%20Name%20Tag%20Structure))
  (Variables|UserInfo|SetPersonalState PersonalState))