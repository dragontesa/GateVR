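; Mirror camera that scene-captures only the player's VR character, framed from sockets on its body mesh.
; InitMirrorCam sets the show-only list and binds to VRIK sit-state changes; Tick snaps the capture to the active socket.
; SetScenePositionNumber cycles head, upper and body framings with matching FOV, attaching a point light at the upper socket.
; The character's body and face join lighting channel 2 until DoDestroy removes the light and camera.
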(event Custom|DoDestroy
  (Utilities|FlowControl|Sequence
    (:then_0
      (bind _pointlight (Variables|Default|GetPointLight)
        (:then
          (Components|DestroyComponent _pointlight))
        (:else)))
    (:then_1
      (CallFunction|SetCharacterLightChannel true true false)
      (Actor|DestroyActor))))

(event EventTick
  (params (DeltaSeconds :type Float%20%28single-precision%29))
  (CallFunction|SetCameraPosition false))

(fn ConstructionScript)

(fn InitMirrorCam
  (params (Parent :type Actor%20Object%20Reference))
  (Variables|Default|SetPlayerCharacterRef Parent)
  (CallFunction|BindEvent)
  (CallFunction|SetShowList)
  (CallFunction|SetAttachParent)
  (CallFunction|SetScenePositionNumber))

(fn SetShowList
  (Rendering|SceneCapture|ShowOnlyActorComponents (Variables|DecalActor|GetCaptureComponent2D) (Variables|Default|GetPlayerCharacterRef) false)
  (CallFunction|SetCharacterLightChannel true true true))

(fn SetAttachParent
  (bind _asbp_gate_character_vr (Utilities|Casting|CastToBP_GateCharacter_VR (Variables|Default|GetPlayerCharacterRef)))
  (Variables|Default|SetAttachParent (Variables|/Game/Multiplayer/Characters/BP_GateCharacter_Base.BP_GateCharacter_Base_C|GetBody _asbp_gate_character_vr)))

(fn SetScenePositionNumber
  (Variables|Default|SetPositionNumber (Math|Integer|SelectInt 0 (+ (Variables|Default|GetPositionNumber) 1) (> (+ (Variables|Default|GetPositionNumber) 1) 2)))
  (Utilities|FlowControl|Sequence
    (:then_0
      (CallFunction|SetCameraPosition false))
    (:then_1
      (Transformation|AttachComponentToComponent (Variables|Default|GetPointLight) (Variables|Default|GetAttachParent) "Socket_CameraPosition_Upper" "SnapToTarget" "KeepRelative" "KeepRelative" true)
      (Variables|/Script/Engine.SceneCaptureComponent2D|SetFOVAngle (Variables|DecalActor|GetCaptureComponent2D) (Utilities|Select :Index (Variables|Default|GetPositionNumber) :Option%200 45.0 :Option%201 45.0 :Option%202 32.5)))))

(fn SetCameraPosition
  (params (IsSit :type Boolean))
  (bind _positionnumber (Variables|Default|GetPositionNumber))
  (bind _returnvalue (Utilities|Select :Index _positionnumber :Option%200 "Socket_CameraPosition_Head" :Option%201 "Socket_CameraPosition_Upper" :Option%202 "Socket_CameraPosition_Body"))
  (bind _attachparent (Variables|Default|GetAttachParent)
    (:then
      (Transformation|SetWorldLocationAndRotation (Variables|DecalActor|GetCaptureComponent2D) (Transformation|GetSocketLocation _attachparent _returnvalue) (Transformation|GetSocketRotation _attachparent _returnvalue) false false))
    (:else)))

(fn BindEvent
  (bind _ref_vrik (Variables|/Game/Multiplayer/Blueprints/BP_GatePlayerController.BP_GatePlayerController_C|GetRef_VRIK (CallFunction|GetGateController))
    (:then
      (EventDispatchers|BindEventtoOnSitStateChanged _ref_vrik (EventDispatchers|CreateEvent :!event SetCameraPosition)))
    (:else)))

(fn ResetCameraPosition
  (Variables|Default|SetPositionNumber -1)
  (CallFunction|SetScenePositionNumber))

(fn SetCharacterLightChannel
  (params (bChannel0 :type Boolean) (bChannel1 :type Boolean) (bChannel2 :type Boolean))
  (bind _asbp_gate_character_vr (Utilities|Casting|CastToBP_GateCharacter_VR (Variables|Default|GetPlayerCharacterRef)))
  (Rendering|Components|SetLightingChannels (Variables|/Game/Multiplayer/Characters/BP_GateCharacter_Base.BP_GateCharacter_Base_C|GetBody _asbp_gate_character_vr) bChannel0 bChannel1 bChannel2))