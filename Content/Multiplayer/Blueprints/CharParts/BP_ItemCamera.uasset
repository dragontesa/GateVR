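; BP_ItemCamera is a scene capture camera that shows only its ShowActor, framing the body or face based on the item part clicked.
; It attaches to the BP_GateCharacter_VR body mesh, using the head socket for face views, and applies a per-view relative transform from a map.
; It moves the character's body and face to lighting channel 2 on BeginPlay and restores channels 0 and 1 in DoDestroy.
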(event Custom|DoDestroy
  (if (not (Game|IsActorBeingDestroyed))
    (CallFunction|SetCharacterLightChannel true true false)
    (Actor|DestroyActor)))

(event EventBeginPlay
  (Rendering|SceneCapture|ShowOnlyActorComponents (Variables|Default|GetSceneCaptureComponent2D) (Variables|Default|GetShowActor) false)
  (CallFunction|SetAttachParent)
  (CallFunction|SetCameraPosition "NewEnumerator0")
  (CallFunction|SetCharacterLightChannel false false true))

(fn ConstructionScript)

(fn SetCameraPosition
  (params (Type :type EDummyCameraType%20Enum :default "NewEnumerator0"))
  (Variables|Default|SetCurrentType Type)
  (switch Utilities|FlowControl|Switch|SwitchonEDummyCameraType (Variables|Default|GetCurrentType)
    (:NewEnumerator0
      (Transformation|AttachComponentToComponent (Variables|Default|GetAttachParent) "None" "KeepRelative" "KeepRelative" "KeepRelative" true))
    (:NewEnumerator1
      (Transformation|AttachComponentToComponent (Variables|Default|GetAttachParent) "head" "KeepRelative" "KeepRelative" "KeepRelative" true)))
  (Transformation|SetRelativeTransform (Variables|Default|GetSceneCaptureComponent2D) (.Value (Utilities|Map|Find (Variables|Components|GetCameraTransformArr) (Variables|Default|GetCurrentType))) false false))

(fn ItemPartsClicked
  (params (PartsType :type String))
  (switch string PartsType
    (:Default
      (CallFunction|SetCameraPosition "NewEnumerator0"))
    (:FM
      (CallFunction|SetCameraPosition "NewEnumerator1" :!label _label))
    (:HA
      (goto _label))))

(fn SetAttachParent
  (bind _asbp_gate_character_vr (Utilities|Casting|CastToBP_GateCharacter_VR (Variables|Default|GetShowActor)))
  (Variables|Default|SetAttachParent (Variables|/Game/Multiplayer/Characters/BP_GateCharacter_Base.BP_GateCharacter_Base_C|GetBody _asbp_gate_character_vr)))

(fn SetCharacterLightChannel
  (params (bChannel0 :type Boolean) (bChannel1 :type Boolean) (bChannel2 :type Boolean))
  (bind _asbp_gate_character_vr (Utilities|Casting|CastToBP_GateCharacter_VR (Variables|Default|GetShowActor)))
  (Rendering|Components|SetLightingChannels (Variables|/Game/Multiplayer/Characters/BP_GateCharacter_Base.BP_GateCharacter_Base_C|GetBody _asbp_gate_character_vr) bChannel0 bChannel1 bChannel2))