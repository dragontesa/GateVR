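; Networked VR selfie camera that shows a live mirror widget from a scene capture render target, with FOV zoom and grab attachment.
; A replicated countdown drives text and sounds, then triggers a capture on the owner.
; Photos export as PNG to the user directory and upload through the gate controller's Socket.IO reference.
; While attached, the owning client sends its transform on a timer and other clients interpolate toward it on Tick.
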(event Custom|FileUpload
  (params (bSuccess :type Boolean))
  ;[1 1 1] FileUpload
  (Default|SendFileUpload (Variables|/Game/Multiplayer/Blueprints/BP_GatePlayerController.BP_GatePlayerController_C|GetSocketIoRef (CallFunction|GetGateController)) 1.0 (Utilities|String|Append (Variables|Default|GetFilePath) ".png") (Utilities|Array|MakeArray "")))

(event Custom|DisableSpotLight
  (bind _asbp_gate_character_vr (Utilities|Casting|CastToBP_GateCharacter_VR (Components|GetOwner)))
  (Rendering|SetVisibility (Variables|/Game/Multiplayer/Characters/BP_GateCharacter_Base.BP_GateCharacter_Base_C|GetSpotLight _asbp_gate_character_vr) false false))

(event EventTick
  (params (DeltaSeconds :type Float%20%28single-precision%29))
  (CallFunction|InterpTransform))

(event EventActorMove
  (params (Value :type Float%20%28double-precision%29))
  ;[1 1 1] Camera Move
  (Transformation|AddActorLocalOffset (Math|Vector|MakeVector Value 0.0 0.0) false false))

(event EventBeginPlay
  (|CallParentFunction)
  (if (Util|IsLocal)
    (Transform|SendTransform)))

(event EventDetachActor
  ;[1 1 1] Camera Move
  (Transformation|DetachFromActor "KeepWorld" "KeepWorld" "KeepWorld")
  (Variables|Default|SetIsAttach false)
  (CallFunction|DisableInterpTransformServer))

(event Custom|StartCaptureCount_Server
  (Count|StartCaptureCount))

(event Custom|Capture_Own
  (Camera|Capture))

(event Custom|SendTransform_Server
  (params (ActorTransform :type Transform))
  (Variables|Default|SetActorTransform ActorTransform))

(event Custom|DisableInterpTransform_All
  (CallFunction|DisableInterpTransform))

(event Custom|SetVisibilityCountText_All
  (params (Visibility :type ESlateVisibility%20Enum :default "Visible"))
  (Default|SetVisibilityCountText (Variables|Default|GetSelfCam_Ref) Visibility))

(event Custom|DisableInterpTransform_Server
  (CallFunction|DisableInterpTransformAll))

(event Custom|ActiveInterpTransform_Server
  (CallFunction|ActiveInterpTransformAll))

(event Custom|ActiveInterpTransform_All
  (CallFunction|ActiveInterpTransform))

(fn ConstructionScript)

(fn Zoomin
  (params (Value :type Float%20%28single-precision%29))
  (if (and (< (+ (Variables|/Script/Engine.SceneCaptureComponent2D|GetFOVAngle (Variables|Default|GetSceneCaptureComponent2D)) Value) 9e+01) (> (+ (Variables|/Script/Engine.SceneCaptureComponent2D|GetFOVAngle (Variables|Default|GetSceneCaptureComponent2D)) Value) 1e+01))
    (Variables|/Script/Engine.SceneCaptureComponent2D|SetFOVAngle (Variables|Default|GetSceneCaptureComponent2D) (+ (Variables|/Script/Engine.SceneCaptureComponent2D|GetFOVAngle (Variables|Default|GetSceneCaptureComponent2D)) Value))))

(fn Capture
  (bind _scenecapturecomponent2d (Variables|Default|GetSceneCaptureComponent2D))
  ;[1 1 1] 미러를 띄워놓은 상태에서 셀카 찍을 때
  (Rendering|SceneCapture|CaptureScene _scenecapturecomponent2d :!class /Script/Engine.SceneCaptureComponent2D)
  (bind _result (CallFunction|GetNowTimetoString false false))
  (bind _output_get (Variables|Default|SetFilename (Utilities|String|Append _result "_" (Utilities|String|ToString(Integer) (Math|Random|RandomIntegerinRange 100000 999999)))))
  (bind _output_get_2 (Variables|Default|SetFilePath (Utilities|String|Append (Utilities|String|Append (Class|KismetSystemLibrary|GetPlatformUserDir) "GateVR/ScreenShot/") _output_get)))
  (Class|ImageWriteBlueprintLibrary|ExporttoDisk (Variables|/Script/Engine.SceneCaptureComponent2D|GetTextureTarget _scenecapturecomponent2d) _output_get_2 (Utilities|Struct|MakeImageWriteOptions "PNG" (EventDispatchers|CreateEvent :!event Custom|FileUpload))) ; Export 할때는 filename에 확장자가 없어도 된다
)

(fn TimetoString
  (bind _returnvalue (Math|DateTime|Now))
  (bind (_year _month _day _hour _minute _second _millisecond) (Math|DateTime|BreakDateTime _returnvalue))
  (return (Utilities|String|Append (Utilities|String|ToString(Integer) _year) "-" (Util|Addnum0 (Utilities|String|ToString(Integer) _month)) "-" (Util|Addnum0 (Utilities|String|ToString(Integer) _day)) " " (Util|Addnum0 (Utilities|String|ToString(Integer) _hour)) "." (Util|Addnum0 (Utilities|String|ToString(Integer) _minute)) "." (Util|Addnum0 (Utilities|String|ToString(Integer) _second)) "." (Utilities|String|ToString(Integer) _millisecond) ".")))

(fn Addnum0
  (params (S :type String))
  (return (Utilities|Select :Index (Utilities|String|Len S) :Option%200 S :Option%201 (Utilities|String|Append "0" S) :Option%202 S)))

(fn StartCaptureCount
  (if (not (Variables|Count|GetIsCount))
    (Utilities|FlowControl|Sequence
      (:then_0
        (Variables|Count|SetIsCount true)
        (Variables|Count|SetCurrentCount (Variables|Count|GetMaxCount)))
      (:then_1
        (CallFunction|SetVisibilityCountTextAll "Visible"))
      (:then_2
        (bind _returnvalue (Utilities|Time|SetTimerbyEvent (EventDispatchers|CreateEvent :!event CountDown) 1.0 true))
        (Variables|Count|SetCameraCountTimerHandle _returnvalue)))))

(fn SetCountText
  (Utilities|FlowControl|Sequence
    (:then_0
      (Default|SetCountText (Variables|Default|GetSelfCam_Ref) (Variables|Count|GetCurrentCount)))
    (:then_1
      (Count|PlayCountSound))))

(fn CountDown
  ;[1 1 1] CountDown
  (bind _output_get (Variables|Count|SetCurrentCount (- (Variables|Count|GetCurrentCount) 1)))
  (if (== _output_get 0)
    (Utilities|FlowControl|Sequence
      (:then_0
        ;[1 1 1] ClearTimer
        (Utilities|Time|ClearandInvalidateTimerbyHandle (Variables|Count|GetCameraCountTimerHandle)))
      (:then_1
        ;[1 1 1] CaptureCam
        (CallFunction|CaptureOwn))
      (:then_2
        ;[1 1 1] ResetValue
        (CallFunction|SetVisibilityCountTextAll "Hidden")
        (Variables|Count|SetIsCount false)))))

(fn PlayCountSound
  (if (== (Variables|Count|GetCurrentCount) 0)
    (Audio|SpawnSoundatLocation "/Game/Sounds/Effect_Sound/HUD/camera_shutter_Cue.camera_shutter_Cue" "0, 0, 0" "0, 0, 0" 0.5 1.0 0.0 0 "/Game/Sounds/Effect_Sound/HUD/Concurrency_HUD.Concurrency_HUD")
    (else
      (Audio|SpawnSoundatLocation (.Value (Utilities|Map|Find (Variables|Count|GetCountDownSound) (Variables|Count|GetCurrentCount))) "0, 0, 0" "0, 0, 0" 1.0 1.0 0.0 0 0))))

(fn SetRenderTarget
  (bind _returnvalue (Rendering|CreateRenderTarget2D 2048 2048 "RTF_RGBA8_SRGB"))
  (bind _output_get (Variables|/Script/Engine.SceneCaptureComponent2D|SetTextureTarget (Variables|Default|GetSceneCaptureComponent2D) _returnvalue))
  (Variables|Default|SetRT_SelfCam _output_get))

(fn InitializeWidget
  (bind _asw_self_cam (Utilities|Casting|CastToW_SelfCam (UserInterface|GetWidget (Variables|Default|GetWidget))))
  (Variables|Default|SetSelfCam_Ref _asw_self_cam)
  (Init|SetRenderTarget)
  (Default|SetMirrorMaterial (Variables|Default|GetSelfCam_Ref) (Variables|Default|GetRT_SelfCam))
  (Utilities|Time|ClearandInvalidateTimerbyHandle (Variables|Default|GetInitWidgetRef_Timer)))

(fn OnRepCurrentCount
  (Count|SetCountText))

(fn SendTransform
  (CallFunction|SendTransformServer (Transformation|GetActorTransform)))

(fn InterpTransform
  (Transformation|SetActorTransform (Class|KismetMathLibrary|TInterpto (Transformation|GetActorTransform) (Variables|Default|GetActorTransform) (Utilities|Time|GetWorldDeltaSeconds) 1e+01)))

(fn ActiveInterpTransform
  (if (Util|IsLocal)
    (bind _returnvalue (Utilities|Time|SetTimerbyEvent (EventDispatchers|CreateEvent :!event SendTransform) 0.1 true))
    (Variables|Default|SetSendTransform_Timer _returnvalue)
    (elif (not (Networking|IsDedicatedServer))
      (Actor|Tick|SetActorTickEnabled true))))

(fn DisableInterpTransform
  (if (Util|IsLocal)
    (Utilities|Time|ClearandInvalidateTimerbyHandle (Variables|Default|GetSendTransform_Timer))
    (else
      (Actor|Tick|SetActorTickEnabled false))))

(fn IsLocal
  (if (Networking|IsDedicatedServer)
    (return false)
    (else
      (bind _aspawn (Utilities|Casting|CastToPawn (Components|GetOwner)))
      (Utilities|IsValid (Pawn|GetController _aspawn)
        (:Is%20Valid
          (return true))
        (:Is%20Not%20Valid
          (return false))))))

(fn DestroyStereoLayer
  (Utilities|IsValid (Class|StereoLayerComponent|GetTexture (Variables|Default|GetStereoLayer))
    (:Is%20Valid
      (Class|StereoLayerComponent|SetTexture (Variables|Default|GetStereoLayer)))
    (:Is%20Not%20Valid
      (CallFunction|DisableSpotLight)
      (Utilities|Time|ClearandInvalidateTimerbyHandle (Variables|Default|GetDestroy_Timer))
      (Actor|SetLifeSpan 0.2))))

(fn AttachActorComp
  (params (Parent :type Scene%20Component%20Object%20Reference))
  (if (== (Components|GetOwner) (Components|GetOwner (Components|GetOwner Parent)))
    (if (Variables|Default|GetIsAttach)
      (return false 0)
      (else
        (Variables|Default|SetIsAttach true)
        (Transformation|AttachComponentToComponent Parent "None" "KeepWorld" "KeepWorld" "KeepWorld" true)
        (CallFunction|ActiveInterpTransformServer)
        (return true self)))))