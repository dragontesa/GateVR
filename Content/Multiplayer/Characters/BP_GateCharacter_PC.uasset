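; BP_GateCharacter_PC is the desktop variant of the multiplayer Gate character, disabling the HMD, removing face tracking and snapping the right motion controller to the camera.
; Enhanced Input movement and legacy axis look pass through GateController mode checks, except pitch, which is only clamped.
; When movement is blocked, mode-specific fallbacks allow chair escape or inverted third-person strafing through VRIK.
; Right-mouse release calls VRIK's server release, and face-tracking functions are empty.
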(event Input|EnhancedActionEvents|EnhancedInputActionIA_T1_MoveRight
  (params (ActionValue :type Float%20%28double-precision%29) (ElapsedSeconds :type Float%20%28double-precision%29) (TriggeredSeconds :type Float%20%28double-precision%29) (InputAction :type Input%20Action%20Object%20Reference :default "/Game/Multiplayer/Input/IA_T1_MoveRight.IA_T1_MoveRight"))
  (:Triggered
    (if (not (Default|IsModeInputBlocked (CallFunction|GetGateController)))
      (CallFunction|InputRight ActionValue))))

(event Input|EnhancedActionEvents|EnhancedInputActionIA_T1_MoveForward
  (params (ActionValue :type Float%20%28double-precision%29) (ElapsedSeconds :type Float%20%28double-precision%29) (TriggeredSeconds :type Float%20%28double-precision%29) (InputAction :type Input%20Action%20Object%20Reference :default "/Game/Multiplayer/Input/IA_T1_MoveForward.IA_T1_MoveForward"))
  (:Triggered
    (if (not (Default|IsModeInputBlocked (CallFunction|GetGateController)))
      (CallFunction|InputForward ActionValue))))

(event EventBeginPlay
  (|CallParentFunction)
  (CallFunction|InputMapping)
  (Class|HeadMountedDisplayFunctionLibrary|EnableHMD false)
  (Components|DestroyComponent (Variables|Default|GetGateXRFaceTracking))
  (Transformation|AttachComponentToComponent (Variables|Default|GetMotionControllerR) (Variables|Default|GetCamera) "None" "SnapToTarget" "SnapToTarget" "KeepWorld" true))

(event Input|AxisEvents|InputAxisLookUp
  (params (AxisValue :type Float%20%28single-precision%29))
  (bind _camera (Variables|Default|GetCamera))
  (bind _relativerotation (Variables|/Script/Engine.SceneComponent|GetRelativeRotation _camera))
  (Transformation|SetRelativeRotation (Variables|Default|GetCamera) (Math|Rotator|MakeRotator (.roll _relativerotation) (Math|Float|ClampAngle (+ (.pitch _relativerotation) (* AxisValue -1.0)) -8e+01 8e+01) (.yaw _relativerotation)) false false))

(event Input|AxisEvents|InputAxisTurn
  (params (AxisValue :type Float%20%28single-precision%29))
  (if (not (Default|IsModeInputBlocked (CallFunction|GetGateController)))
    (CallFunction|InputTurning AxisValue)))

(event Input|MouseEvents|RightMouseButton
  (params (Key :type Key%20Structure :default "None"))
  (:Released
    (bind _vrik (Variables|Default|GetVRIK)
      (:then
        (Default|TryReleaseServer _vrik false))
      (:else))))

(fn ConstructionScript
  (|CallParentFunction))

(fn InputForward
  (params (Value :type Float%20%28double-precision%29))
  (bind _controller (CallFunction|GetGateController))
  (bind _controller_2 (CallFunction|GetGateController))
  (if (or (Default|IsModeMoveBlocked _controller) (Default|IsModeInputBlocked _controller))
    (if (Default|IsModeSame (CallFunction|GetGateController) "NewEnumerator4")
      (bind _output_get (Variables|Default|SetMoveInput_Y Value :!label _label))
      (Default|CallInputMoveForward _output_get)
      (else
        (Variables|Default|SetMoveInput_Y 0.0)
        (if (not (Variables|/Game/Multiplayer/Blueprints/BP_GatePlayerController.BP_GatePlayerController_C|GetIsStandingDisable _controller_2))
          (if (Default|IsModeSame _controller_2 "NewEnumerator10")
            (if (> (Math|Float|Absolute(Float) Value) 0.5)
              (bind _vrik (Variables|Default|GetVRIK)
                (:then
                  (if (Variables|/Game/Animations/VRFBIK/V2/BP_VRIK_V2.BP_VRIK_V2_C|GetIsOnStation _vrik)
                    (Default|EscapeonChair _vrik)))
                (:else)))))))
    (else
      (goto _label))))

(fn InputTurning
  (params (Value :type Float%20%28double-precision%29))
  (bind _camera (Variables|Default|GetCamera))
  (bind _relativerotation (Variables|/Script/Engine.SceneComponent|GetRelativeRotation _camera))
  (if (not (Default|IsModeInputBlocked (CallFunction|GetGateController)))
    (if (Default|IsModeMoveBlocked (CallFunction|GetGateController))
      (if (not (Default|IsModeSame (CallFunction|GetGateController) "NewEnumerator4"))
        (Transformation|SetRelativeRotation (Variables|Default|GetCamera) (Math|Rotator|MakeRotator (.roll _relativerotation) (.pitch _relativerotation) (+ (.yaw _relativerotation) Value)) false false :!label _label))
      (else
        (Default|CallInputTurn Value)
        (goto _label)))))

(fn InputRight
  (params (Value :type Float%20%28double-precision%29))
  (bind _controller (CallFunction|GetGateController))
  (if (or (Default|IsModeMoveBlocked _controller) (Default|IsModeInputBlocked _controller))
    (if (Default|IsModeSame (CallFunction|GetGateController) "NewEnumerator4")
      (bind _output_get (Variables|Default|SetMoveInput_X Value :!label _label))
      (Default|CallInputMoveRight _output_get)
      (else
        (Variables|Default|SetMoveInput_X 0.0)
        (if (not (Default|IsModeSame (CallFunction|GetGateController) "NewEnumerator8"))
          (bind _vrik (Variables|Default|GetVRIK)
            (:then
              (if (Variables|/Game/Animations/VRFBIK/V2/BP_VRIK_V2.BP_VRIK_V2_C|GetIsThirdPerson _vrik)
                (Default|CallInputMoveRight (* Value -1))))
            (:else)))))
    (else
      (goto _label))))

(fn InputMapping
  (bind _returnvalue (Game|GetPlayerController 0))
  (bind _returnvalue_2 (PlayerController|LocalPlayerSubsystems|GetEnhancedInputLocalPlayerSubsystem _returnvalue))
  (Utilities|IsValid _returnvalue_2
    (:Is%20Valid
      (Input|AddMappingContext _returnvalue_2 "/Game/Multiplayer/Input/IMC_Default_MP.IMC_Default_MP" 0 "(bIgnoreAllPressedKeysUntilRelease=True,bForceImmediately=False)"))))

(fn UpdateFaceExpression)

(fn SendFaceExpression)

(fn InitFaceTracking)