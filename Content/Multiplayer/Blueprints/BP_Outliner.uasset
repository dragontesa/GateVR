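; BP_Outliner manages outlines on nearby interactable actors in the local player's view, limiting how many are highlighted.
; BeginPlay starts a looping one-second timer, while UpdateOutliner gathers non-spawner interaction-interface actors within view angle and camera range.
; It sorts candidates by camera distance and enables outlines only on the closest ActiveAmount.
; Actors failing the filter lose their outline unless hovered.
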(event EventBeginPlay
  (CallFunction|BeginOutliner))

(fn ConstructionScript)

(fn BeginOutliner
  (bind _returnvalue (Utilities|Time|SetTimerbyEvent (EventDispatchers|CreateEvent :!event UpdateOutliner) 1.0 true))
  (Variables|Default|SetOutliner_Timer _returnvalue))

(fn UpdateOutliner
  (Utilities|FlowControl|Sequence
    (:then_0
      (bind _outactors (Actor|GetAllActorswithInterface "/Game/LevelDesign/Assets/Blueprints/BP_Interface_InteractionActor.BP_Interface_InteractionActor_C"))
      (for _array_element _outactors
        (bind _isspawn (Class|BPInterfaceInteractionActor|IsSpawner(Message) _array_element))
        (if (Math|Boolean|ANDBoolean (not _isspawn) (CallFunction|IsTargetinLocalView (Variables|/Script/Engine.Actor|GetRootComponent _array_element) (LocalVariables|GetViewAngle)) (CallFunction|IsTargetinRange (Variables|/Script/Engine.Actor|GetRootComponent _array_element) (Camera|GetCameraLocation (Game|GetPlayerCameraManager 0)) (LocalVariables|GetViewRange)))
          (Utilities|Array|Add (LocalVariables|GetList) _array_element)
          (else
            (bind _ishover (Class|BPInterfaceInteractionActor|IsHovering(Message) _array_element))
            (if (not _ishover)
              (Class|BPInterfaceInteractionActor|SetOutlineEnable(Message) _array_element false))))))
    (:then_1
      (for (_array_element_2 _array_index) (CallFunction|SortActorsClosest (LocalVariables|GetList) (Camera|GetCameraLocation (Game|GetPlayerCameraManager 0)))
        (if (< _array_index (LocalVariables|GetActiveAmount))
          (Class|BPInterfaceInteractionActor|SetOutlineEnable(Message) _array_element_2 true)
          (else
            (Class|BPInterfaceInteractionActor|SetOutlineEnable(Message) _array_element_2 false)))))))