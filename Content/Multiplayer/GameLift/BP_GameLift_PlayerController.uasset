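; GameLift multiplayer player controller that passes room player count and map to the server game mode.
; On non-dedicated BeginPlay, match-join clients send a zero count with a random chat level, while hosts send the gate instance's count and map.
; The user-count event forwards these values to BP_GameLift_ServerGameMode's SetRoomInfo.
; InitialSetup reloads saved GameLift session, player-session and fleet IDs, then re-saves them with a flag set true.
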(event Custom|InitialSetup
  ;[1 1 1] Setup
  (bind _loadedgameliftplayerinfo (CallFunction|LoadGameLiftPlayerInfo))
  (bind _output_get (Variables|Default|SetGameLiftPlayerInfo (Utilities|Struct|MakeBP_GameLift_PlayerInfo (.Player_GameSessionId (Utilities|Struct|BreakBP_GameLift_PlayerInfo _loadedgameliftplayerinfo)) (.Player_PlayerSessionId (Utilities|Struct|BreakBP_GameLift_PlayerInfo _loadedgameliftplayerinfo)) (.Player_FleetId (Utilities|Struct|BreakBP_GameLift_PlayerInfo _loadedgameliftplayerinfo)) true)))
  (CallFunction|SaveGameLiftPlayerInfo _output_get))

(event Custom|Check_UserCount
  (params (RoomPlayerCount :type Integer) (MapName :type String))
  ;[0.1329 0.1912 0.2705] Start Count Players Joined in Only Room Host
  (bind _asbp_game_lift_server_game_mode (Utilities|Casting|CastToBP_GameLift_ServerGameMode (Game|GetGameMode)))
  (Default|SetRoomInfo _asbp_game_lift_server_game_mode RoomPlayerCount MapName))

(event EventBeginPlay
  (bind _instance (CallFunction|GetGateInstance))
  (bind _mapname (Variables|/Game/Multiplayer/Blueprints/BP_GateGameInstance.BP_GateGameInstance_C|GetMapName _instance))
  ;[1 1 1] CheckUserCount
  (if (not (Networking|IsDedicatedServer))
    (if (Variables|/Game/Multiplayer/Blueprints/BP_GateGameInstance.BP_GateGameInstance_C|GetIsJoinMatchServer _instance)
      (CallFunction|CheckUserCount 0 (CallFunction|GetRandomChatLevel))
      (Development|PrintString "JoinMatchingRoom")
      (elif (Variables|/Game/Multiplayer/Blueprints/BP_GateGameInstance.BP_GateGameInstance_C|GetIsHost _instance)
        (CallFunction|CheckUserCount (Variables|/Game/Multiplayer/Blueprints/BP_GateGameInstance.BP_GateGameInstance_C|GetUserCount _instance) _mapname)
        (Development|PrintString (Utilities|String|Append "Join : " _mapname) true true "(R=0.000000,G=0.660000,B=1.000000,A=1.000000)" 1e+01)))))

(fn ConstructionScript)

(fn GetRandomChatLevel
  (bind _frandomchatlevellist (Utilities|Struct|MakeFRandomChatLevelList))
  (return (Utilities|Array|Get(acopy) (.list_levelname _frandomchatlevellist) (Math|Random|RandomInteger (Utilities|Array|Length (.list_levelname _frandomchatlevellist))))))