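; Voice translation component for XL8-based multiplayer talk, with nearly all event and talk logic currently disabled.
; The disabled Tick toggles audio recording on a single-eye wink, detected as a peak-then-fall in Oculus XR face expression values.
; The disabled translation callback sends speaker ID and sentence to a lazily spawned balloon talk HUD.
; Countdown and toast HUD helpers remain enabled, while StartTalking and StopTalking have disabled bodies.
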(event Custom|OnVoiceTranslated
  (params (success :type Boolean) (sentence :type String) (UserId :type String))
  (bind _returnvalue (Utilities|String|Append UserId " : " sentence))
  ;[0.03071 0.06848 0.2705] Handle the result to translate a voice speech.
  (if success
    (bind _talkhudref (CallFunction|BalloonTalkHud))
    (Default|OnInputTalkWords _talkhudref (Utilities|String|Replace _returnvalue "(part)"))
    (Development|PrintString _returnvalue true true "(R=0.141854,G=0.744792,B=0.000000,A=1.000000)" 1e+01)
    (else
      (Development|PrintString "XL8 Translate Failure!"))))

(event EventBeginPlay
  (bind _asbp_gate_character_vr (Utilities|Casting|CastToBP_GateCharacter_VR (Game|GetPlayerCharacter 0)))
  (Variables|Default|SetPlayerFaceExpCharacterRef _asbp_gate_character_vr))

(event EventTick
  (params (DeltaSeconds :type Float%20%28single-precision%29))
  ;[0.03071 0.06848 0.2705] Aware of a face expression, here is for Wink, then use that to toggle audio recording
  (Utilities|FlowControl|Sequence
    (:then_0
      (bind (_isdetected _isdetectstarted _updatedvalue) (CallFunction|DetectExpression (Utilities|Enum|LiteralenumEOculusXRFaceExpression "EyesClosedL") 0.65 (Variables|Default|GetOldLeftEyeClosedValue) (Variables|Default|GetIsLeftEyeDetectStarted)))
      (if _isdetected
        (Variables|Default|SetIsLeftEyeDetectStarted false)
        (Variables|Default|SetOldLeftEyeClosedValue 0.0)
        (Variables|Default|SetBothEyeClosedState (Class|KismetMathLibrary|OrIntInt (Variables|Default|GetBothEyeClosedState) 1))
        (else
          (Variables|Default|SetIsLeftEyeDetectStarted _isdetectstarted)
          (Variables|Default|SetOldLeftEyeClosedValue _updatedvalue))))
    (:then_1
      (bind (_isdetected_2 _isdetectstarted_2 _updatedvalue_2) (CallFunction|DetectExpression (Utilities|Enum|LiteralenumEOculusXRFaceExpression "EyesClosedR") 0.65 (Variables|Default|GetOldRightEyeClosedValue) (Variables|Default|GetIsRightEyeDetectStarted)))
      (if _isdetected_2
        (Variables|Default|SetIsRightEyeDetectStarted false)
        (Variables|Default|SetOldRightEyeClosedValue 0.0)
        (Variables|Default|SetBothEyeClosedState (Class|KismetMathLibrary|OrIntInt (Variables|Default|GetBothEyeClosedState) 2))
        (else
          (Variables|Default|SetIsRightEyeDetectStarted _isdetectstarted_2)
          (Variables|Default|SetOldRightEyeClosedValue _updatedvalue_2))))
    (:then_2
      (if (and (> (Variables|Default|GetBothEyeClosedState) 0) (!= (Variables|Default|GetBothEyeClosedState) 3))
        (bind _output_get (Variables|Default|SetIsAudioRecording (not (Variables|Default|GetIsAudioRecording))))
        (CallFunction|StartAudioRecording _output_get))
      (Variables|Default|SetBothEyeClosedState 0))
    (:then_3
      (bind _output_get_2 (Variables|Default|SetDebugElapsed (+ DeltaSeconds (Variables|Default|GetDebugElapsed))))
      (if (> _output_get_2 1.0)
        (Development|PrintText (Utilities|Text|FormatText "Audio Sampling is { enabled }" (Variables|Default|GetIsAudioRecording)) true true "(R=1.000000,G=0.102869,B=0.815589,A=1.000000)" 1.0)
        (Variables|Default|SetDebugElapsed 0.0)
        (elif (> (Variables|Default|GetDebugElapsed) 0.1)
          (Development|PrintText (Utilities|Text|FormatText "left_eyeclose={val}" (Variables|Default|GetOldLeftEyeClosedValue))))))))

(fn BalloonTalkHud
  (Variables|Default|GetBallonTalkHudRef
    (:then
      _)
    (:else
      (bind _returnvalue (Game|SpawnActorfromClass "/Game/XHUD/GateTalkingFreeByXL8/BP_TalkHUD.BP_TalkHUD_C" (Math|Transform|MakeTransform "0, 0, 0" "0, 0, 0" "1.000000,1.000000,1.000000") "AlwaysSpawn" "OverrideRootScale" 0 0))
      (Variables|Default|SetBallonTalkHudRef _returnvalue)))
  (return (Variables|Default|GetBallonTalkHudRef)))

(fn DetectExpression
  (params (ExpressionType :type EOculusXRFaceExpression%20Enum :default "BrowLowererL") (MinimumTopValue :type Float%20%28double-precision%29) (OldExpressionValue :type Float%20%28double-precision%29) (IsDetectStart :type Boolean))
  (LocalVariables|SetUpdatedExpressionValue (Utilities|Array|Get(acopy) (Variables|/Game/Multiplayer/Characters/FBIK/BP_GateCharacter_VR.BP_GateCharacter_VR_C|GetFaceExpression (Variables|Default|GetPlayerFaceExpCharacterRef)) (Math|Conversions|ToInteger(Byte) ExpressionType)))
  (if IsDetectStart
    (return (and (> (- OldExpressionValue (LocalVariables|GetUpdatedExpressionValue)) 0.0) (> OldExpressionValue MinimumTopValue)) true (LocalVariables|GetUpdatedExpressionValue))
    (else
      (bind _output_get (LocalVariables|SetDetectStarted (> (LocalVariables|GetUpdatedExpressionValue) 0.0)))
      (return false _output_get (LocalVariables|GetUpdatedExpressionValue)))))

(fn ShowCountdown
  (bind _countdownprogressref (Variables|Default|GetCountdownProgressRef)
    (:then
      (Default|DoDestroy _countdownprogressref))
    (:else
      _))
  (bind _returnvalue (Game|SpawnActorfromClass "/Game/XHUD/GateTalkingFreeByXL8/BP_CountingProgressHUD.BP_CountingProgressHUD_C" (Math|Transform|MakeTransform "0, 0, 0" "0, 0, 0" "1.000000,1.000000,1.000000") "Undefined" "OverrideRootScale" 0 0))
  (bind _output_get (Variables|Default|SetCountdownProgressRef _returnvalue))
  (return _output_get))

(fn ShowToastMessage
  (params (Message :type String))
  (bind _returnvalue (Game|SpawnActorfromClass "/Game/XHUD/GateTalkingFreeByXL8/BP_ToastMessageHUD.BP_ToastMessageHUD_C" (Math|Transform|MakeTransform "0, 0, 0" "0, 0, 0" "1.000000,1.000000,1.000000") "Undefined" "OverrideRootScale" 0 0))
  (Default|ToastMessage _returnvalue Message))

(fn StartTalking
  (CallFunction|StartAudioRecording true)
  (Variables|Default|SetIsAudioRecording true)
  (Variables|Default|SetisPending true))

(fn StopTalking
  (CallFunction|StartAudioRecording false)
  (Variables|Default|SetIsAudioRecording false)
  (Variables|Default|SetisPending false))