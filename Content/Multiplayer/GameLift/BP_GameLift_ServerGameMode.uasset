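; GameLift multiplayer server game mode that gathers joining players in a session, then moves them to the game map.
; PostLogin records each controller and runs its initial setup.
; SetRoomInfo stores player count and map, then starts a polling timer that triggers travel when enough players join or a force-start timeout expires.
; A delayed timer handles travel, with ServerTravel building the servertravel console command from the map name.
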(event Custom|TravelGame
  ;[0.1329 0.1912 0.2705] Start Travel into The Game
  (bind _returnvalue (Utilities|Time|SetTimerbyEvent (EventDispatchers|CreateEvent :!event ServerTravel) 6.0))
  (Variables|Count|SetServerTravel_TimerHandle _returnvalue))

(event EventPostLogin
  (params (NewPlayer :type Player%20Controller%20Object%20Reference))
  ;[0.1329 0.1912 0.2705] Add a New Player Joined in The Session
  (Utilities|Array|Add (Variables|Players|GetAllPlayerControllers) NewPlayer)
  (bind _asbp_game_lift_player_controller (Utilities|Casting|CastToBP_GameLift_PlayerController NewPlayer))
  (Default|InitialSetup _asbp_game_lift_player_controller))

(fn ConstructionScript)

(fn CheckJoinPlayerCount
  (if (>= (Utilities|Array|Length (Variables|Players|GetAllPlayerControllers)) (Variables|RoomInfo|GetPlayerNumbers))
    (CallFunction|StartTravelIntoGame)
    (Utilities|Time|ClearandInvalidateTimerbyHandle (Variables|Count|GetCheckJoinPlayerCount_TimeHandle))
    (elif (CallFunction|CheckForceStart)
      (CallFunction|StartTravelIntoGame)
      (Utilities|Time|ClearandInvalidateTimerbyHandle (Variables|Count|GetCheckJoinPlayerCount_TimeHandle)))))

(fn SetRoomInfo
  (params (PlayerNumbers :type Integer) (MapName :type String))
  (if (not (Utilities|Time|IsValidTimerHandle (Variables|Count|GetServerTravel_TimerHandle)))
    (Variables|RoomInfo|SetPlayerNumbers PlayerNumbers)
    (Variables|RoomInfo|SetMapName MapName)
    (bind _returnvalue (Utilities|Time|SetTimerbyEvent (EventDispatchers|CreateEvent :!event CheckJoinPlayerCount) 0.1 true))
    (Variables|Count|SetCheckJoinPlayerCount_TimeHandle _returnvalue)
    (Variables|Count|SetForceStartCount 0.0)))

(fn ServerTravel
  (Development|ExecuteConsoleCommand (Utilities|String|Append "servertravel " (Variables|RoomInfo|GetMapName)) 0))

(fn CheckForceStart
  (bind _output_get (Variables|Count|SetForceStartCount (+ (Variables|Count|GetForceStartCount) 0.1)))
  (return (>= _output_get 1e+01)))