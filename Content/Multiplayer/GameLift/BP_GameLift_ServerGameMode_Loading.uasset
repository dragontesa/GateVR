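; GameLift server game mode for a loading map, showing a loading screen to connecting players.
; On PostLogin it runs the parent logic, then spawns a single BP_LoadingScreenHUD actor at a fixed, slightly scaled transform, reusing it if one already exists.
; A separate SetLoadingImage function passes the map name to that actor through its server call to set the image.
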(event EventPostLogin
  (params (NewPlayer :type Player%20Controller%20Object%20Reference))
  (|CallParentFunction NewPlayer)
  (CallFunction|SpawnLoadingImage))

(fn ConstructionScript
  (|CallParentFunction))

(fn SpawnLoadingImage
  (Variables|Default|GetLoadingImage_Ref
    (:then)
    (:else
      (bind _returnvalue (Game|SpawnActorfromClass "/Game/XHUD/Loading/BP_LoadingScreenHUD.BP_LoadingScreenHUD_C" (Math|Transform|MakeTransform "200.000000,0.000000,190.000000" "0, 0, 0" "1.200000,1.200000,1.200000") "Undefined" "MultiplyWithRoot" 0 0))
      (Variables|Default|SetLoadingImage_Ref _returnvalue))))

(fn SetLoadingImage
  (Default|SetLoadingImageServer (Variables|Default|GetLoadingImage_Ref) (Variables|Default|GetMapName)))