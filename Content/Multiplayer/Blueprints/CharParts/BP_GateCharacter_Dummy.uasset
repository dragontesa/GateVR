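; Preview dummy character whose SceneCaptureComponent2D frames either the body or the face according to the clicked item part.
; FM and HA parts select the face view and all others the body view.
; SetCameraPosition reattaches the capture to the mesh or its head socket, applies a mapped transform, and runs ABP_NPC for body view but clears it for face view.
; The actor unhides once after its first item update finishes.
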(event Custom|FinishItemUpdate
  (Utilities|FlowControl|DoOnce false
    (:Completed
      (Rendering|SetActorHiddenInGame false))))

(fn ConstructionScript
  (|CallParentFunction))

(fn SetCameraPosition
  (params (Type :type EDummyCameraType%20Enum :default "NewEnumerator0"))
  (Variables|Default|SetCurrentType Type)
  (switch Utilities|FlowControl|Switch|SwitchonEDummyCameraType (Variables|Default|GetCurrentType)
    (:NewEnumerator0
      (Transformation|AttachComponentToComponent (Variables|Default|GetSceneCaptureComponent2D) (Variables|Default|GetBody) "" "KeepRelative" "KeepRelative" "KeepRelative" true)
      (Class|SkeletalMeshComponent|SetAnimClass (Variables|Default|GetBody) "/Game/Animations/NPC/ABP_NPC.ABP_NPC_C"))
    (:NewEnumerator1
      (Transformation|AttachComponentToComponent (Variables|Default|GetSceneCaptureComponent2D) (Variables|Default|GetBody) "head" "KeepRelative" "KeepRelative" "KeepRelative" true)
      (Class|SkeletalMeshComponent|SetAnimClass (Variables|Default|GetBody))))
  (Transformation|SetRelativeTransform (Variables|Default|GetSceneCaptureComponent2D) (.Value (Utilities|Map|Find (Variables|Default|GetCameraTransformArr) (Variables|Default|GetCurrentType))) false false))

(fn ItemPartsClicked
  (params (PartsType :type String))
  (switch string PartsType
    (:Default
      (CallFunction|SetCameraPosition "NewEnumerator0"))
    (:FM
      (CallFunction|SetCameraPosition "NewEnumerator1" :!label _label))
    (:HA
      (goto _label))))