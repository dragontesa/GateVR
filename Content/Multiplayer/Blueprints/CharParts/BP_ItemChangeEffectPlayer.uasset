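; BP_ItemChangeEffectPlayer is a short-lived actor that plays a visual effect on character materials, apparently for item changes.
; On BeginPlay it caches the dynamic instances from its Materials array and enables their Dissolve_On parameter.
; It spawns a Niagara spark system at EffectSpawnPoint while a timeline drives the Character_Fresnel parameter across those materials.
; When the timeline finishes, it switches Dissolve_On off and destroys itself.
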(event Custom|Fresnel
  (bind _effectspawnpoint (Variables|Default|GetEffectSpawnPoint))
  (Niagara|SpawnSystematLocation "/Game/VFX/Niagara/Niagara_System/Sparks/NS_Spawn_Sparks_04.NS_Spawn_Sparks_04" (.location _effectspawnpoint) (Math|Rotator|MakeRotator 0.0 0.0 (.yaw (.rotation _effectspawnpoint))))
  (bind _alpha (Timeline|Timeline_Fresnel PlayFromStart)
    (:Update
      (for _array_element (Variables|Default|GetMaterialInstanceDynamics)
        (Rendering|Material|SetScalarParameterValue _array_element "Character_Fresnel" _alpha :!class /Script/Engine.MaterialInstanceDynamic)))
    (:Finished
      (for _array_element_2 (Variables|Default|GetMaterialInstanceDynamics)
        (Rendering|Material|SetScalarParameterValue _array_element_2 "Dissolve_On" 0.0 :!class /Script/Engine.MaterialInstanceDynamic))
      (CallFunction|DoDestroyed))))

(event Custom|PreparationFresnel
  (for _array_element (Variables|Default|GetMaterials)
    (bind _asmaterial_instance_dynamic (Utilities|Casting|CastToMaterialInstanceDynamic _array_element))
    (Utilities|Array|Add (Variables|Default|GetMaterialInstanceDynamics) _asmaterial_instance_dynamic)
    (Rendering|Material|SetScalarParameterValue _asmaterial_instance_dynamic "Dissolve_On" 1.0 :!class /Script/Engine.MaterialInstanceDynamic))
  (CallFunction|Fresnel))

(event Custom|DoDestroyed
  (if (not (Game|IsActorBeingDestroyed))
    (Actor|DestroyActor)))

(event EventBeginPlay
  (CallFunction|PreparationFresnel))

(fn ConstructionScript)