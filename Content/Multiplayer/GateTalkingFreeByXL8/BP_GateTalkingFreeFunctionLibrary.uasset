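; Blueprint function library for GateTalkingFree, an XL8 voice translation integration for multiplayer Agora voice chat.
; Initialization calls the GateTalkingfree init, returns true on success and prints an error on failure.
; Release, start and stop logic is all disabled.
; The disabled start path adds a component to the target actor, registers it as translator and Agora audio-frame observer, and binds a translated-voice event.
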(fn InitTalkingFree)

(fn ReleaseTalkingFree)

(fn StartTalkingFree
  (params (TargetActor :type Actor%20Object%20Reference))
  (bind _returnvalue (Game|AddComponentbyClass TargetActor 0))
  (LocalVariables|SetCompRef 0 _returnvalue)
  (bind _returnvalue_2 (CallFunction|InstanceGateTalkingfree))
  (CallFunction|RegisterTranslator _returnvalue _returnvalue_2)
  (CallFunction|SetisfyTranslateRequester _returnvalue)
  (CallFunction|RegisterAgoraAudioFrameObserver _returnvalue (Variables|/Game/Multiplayer/Blueprints/BP_GateGameInstance.BP_GateGameInstance_C|GetRtcEngine_Ref (CallFunction|GetGateInstance)))
  (EventDispatchers|BindEventtoOnVoiceTranslated _returnvalue_2 (EventDispatchers|CreateEvent _returnvalue :!event OnVoiceTranslated))
  (return))

(fn StopTalkingFree
  (bind _returnvalue (CallFunction|TranslateRequester))
  (EventDispatchers|UnbindEventfromOnStreamMessage (Variables|/Game/Multiplayer/Blueprints/BP_GateGameInstance.BP_GateGameInstance_C|GetRtcEngine_EventHandle (CallFunction|GetGateInstance)) (EventDispatchers|CreateEvent _returnvalue :!event OnAgoraStreamMessage)))