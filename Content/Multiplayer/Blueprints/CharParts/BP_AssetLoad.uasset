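; BP_AssetLoad is a short-lived helper actor that loads a character item's class by folder and asset name under /Game/ItemData.
; A looping 0.1-second timer drives retries of an Asset Registry lookup, whose result gets a "_C" suffix for a blocking class load.
; Success broadcasts OnLoadFinish with the class, item and character context, then destroys the actor.
; Repeated failures destroy it without broadcasting.
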(event Custom|LoadAsset
  (bind _outassetdata (Class|AssetRegistry|GetAssetsbyPackageName (Class|AssetRegistryHelpers|GetAssetRegistry) (Utilities|String|StringToName (Utilities|String|Replace (Utilities|String|Append "/Game/ItemData/" (Variables|Default|GetFolderName) "/" (Variables|Default|GetAssetName)) " ")) false true))
  (Variables|Default|SetOutAssetData _outassetdata)
  (Utilities|IsValid (Class|AssetRegistryHelpers|GetAsset (Utilities|Array|Get(acopy) (Variables|Default|GetOutAssetData)))
    (:Is%20Valid
      (bind _returnvalue (Utilities|LoadClassAssetBlocking (Class|KismetSystemLibrary|ToSoftClassRef(SoftClassPath) (Class|KismetSystemLibrary|MakeSoftClassPath (select (Utilities|Enum|Equal(Enum) (Utilities|String|Right (Class|KismetSystemLibrary|GetPathName (Class|AssetRegistryHelpers|GetAsset (Utilities|Array|Get(acopy) (Variables|Default|GetOutAssetData)))) 2) "_C") (Class|KismetSystemLibrary|GetPathName (Class|AssetRegistryHelpers|GetAsset (Utilities|Array|Get(acopy) (Variables|Default|GetOutAssetData)))) (Utilities|String|Append (Class|KismetSystemLibrary|GetPathName (Class|AssetRegistryHelpers|GetAsset (Utilities|Array|Get(acopy) (Variables|Default|GetOutAssetData)))) "_C"))))))
      (Default|CallOnLoadFinish _returnvalue (Variables|Default|GetItemType) (Variables|Default|GetCode) (Variables|Default|GetIsWear) (Variables|Default|GetIsItemChange) (Variables|Default|GetCharacter))
      (CallFunction|DoDestroy))
    (:Is%20Not%20Valid
      (bind _result (Math|Integer|IncrementInt (Variables|Default|GetTryCount))
        (:%20%20
          (if (> _result 10)
            (CallFunction|DoDestroy)))))))

(event Custom|DoDestroy
  (Utilities|Time|ClearandInvalidateTimerbyHandle (Variables|Default|GetAssetLoad_Timer))
  (Actor|DestroyActor))

(event EventBeginPlay
  (bind _returnvalue (Utilities|Time|SetTimerbyEvent (EventDispatchers|CreateEvent :!event Custom|LoadAsset) 0.1 true))
  (Variables|Default|SetAssetLoad_Timer _returnvalue))

(fn ConstructionScript)