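; Socket.IO event handler for the character select screen, relaying web server messages to the game through event dispatchers.
; The select-character event fires once, requesting user info and broadcasting the character preset code to load.
; User-info JSON is unpacked into a character code and parts struct of clothing and appearance fields, then broadcast.
; Enter-world and exit events broadcast level travel plus their own dispatcher, with a button sound on entry.
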(event Custom|s-select-character
  (params (EventData :type SIO%20Json%20Value%20Object%20Reference))
  ;[1 1 1] Sent Event from Web Server
  (Utilities|FlowControl|DoOnce false
    (:Completed
      (CallFunction|SendReqUserInfo)
      (Default|CallOnResponseCharacterLoad (Class|BlueprintJsonLibrary|ToString(JsonValue) (CallFunction|JsontoValue EventData "character_preset_code"))))))

(fn ConstructionScript
  (|CallParentFunction))

(fn S-user-info
  (params (Input :type SIO%20Json%20Value%20Object%20Reference))
  (Default|CallOnResponseUserInfo (Class|BlueprintJsonLibrary|ToString(JsonValue) (CallFunction|JsontoValue Input "character")) (Utilities|Struct|MakeFPartsInfo (Class|BlueprintJsonLibrary|ToString(JsonValue) (CallFunction|JsontoValue Input "Set")) (Class|BlueprintJsonLibrary|ToString(JsonValue) (CallFunction|JsontoValue Input "UpOut")) (Class|BlueprintJsonLibrary|ToString(JsonValue) (CallFunction|JsontoValue Input "UpIn")) (Class|BlueprintJsonLibrary|ToString(JsonValue) (CallFunction|JsontoValue Input "LowOut")) (Class|BlueprintJsonLibrary|ToString(JsonValue) (CallFunction|JsontoValue Input "LowIn")) (Class|BlueprintJsonLibrary|ToString(JsonValue) (CallFunction|JsontoValue Input "Acce")) (Class|BlueprintJsonLibrary|ToString(JsonValue) (CallFunction|JsontoValue Input "Effect")) (Class|BlueprintJsonLibrary|ToString(JsonValue) (CallFunction|JsontoValue Input "Face")) (Class|BlueprintJsonLibrary|ToString(JsonValue) (CallFunction|JsontoValue Input "Feet")) (Class|BlueprintJsonLibrary|ToString(JsonValue) (CallFunction|JsontoValue Input "Hair")))))

(fn S-enter-world
  (params (InputPin :type SIO%20Json%20Value%20Object%20Reference))
  (Default|CallOnLevelTravel)
  (Audio|PlaySound2D "/Game/Sounds/Effect_Sound/Button/Cue_Button_02.Cue_Button_02" 0.5 1.0 0.0 0 0)
  (Default|CallOnEnterWorld))

(fn S-exit-gatevr
  (params (InputPin :type SIO%20Json%20Value%20Object%20Reference))
  (Default|CallOnLevelTravel)
  (Default|CallOnExitGame))