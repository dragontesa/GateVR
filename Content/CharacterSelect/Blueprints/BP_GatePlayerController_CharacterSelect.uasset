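; Player controller for the VR character select level, which opens a stereo web-view character page in front of the pawn and fixes the camera height.
; A local-only SocketIO actor exposes character-load and user-info responses through bound events.
; Character loading stores code and code-derived gender in the game instance and spawns an asset loader.
; Other functions spawn a scaled preview NPC at a spawn point and open the lobby level.
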(event EventBeginPlay
  (|CallParentFunction)
  (HUD|SpawnCharSelectHUD)
  (CallFunction|SetCameraPosition))

(event EventTick
  (params (DeltaSeconds :type Float%20%28single-precision%29))
  (|CallParentFunction DeltaSeconds) ; This node is disabled and will not be called.\nDrag off pins to build functionality.
)

(fn ConstructionScript
  (|CallParentFunction))

(fn StartLevelLoad)

(fn OpenLobbyLevel
  (Default|OpenLevel (CallFunction|GetGateInstance) "A5_001_A_00_P"))

(fn SocketIOBindEvent
  (|CallParentFunction)
  (bind _asbp_socket_io_character_select (Utilities|Casting|CastToBP_SocketIO_CharacterSelect (Variables|Default|GetSocketIoRef)))
  (EventDispatchers|BindEventtoOnResponseCharacterLoad _asbp_socket_io_character_select (EventDispatchers|CreateEvent :!event LoadCharacterSet))
  (EventDispatchers|BindEventtoOnResponseUserInfo _asbp_socket_io_character_select (EventDispatchers|CreateEvent (CallFunction|GetGateInstance) :!event SetUserInfo)))

(fn SpawnCharSelectHUD
  (bind _returnvalue (Game|Player|GetPlayerPawn 0))
  (bind _returnvalue_2 (Transformation|GetActorRotation _returnvalue))
  (bind _returnvalue_3 (Math|Rotator|MakeRotator 0.0 0.0 (.yaw _returnvalue_2)))
  (Variables|Default|GetRef_CharSelect_HUD
    (:then)
    (:else
      (bind _returnvalue_4 (Game|SpawnActorfromClass "/Game/XHUD/BP_StereoWebViewHUD.BP_StereoWebViewHUD_C" (Math|Transform|MakeTransform (+ (Transformation|GetActorLocation _returnvalue) (* (Math|Vector|GetForwardVector _returnvalue_3) 2.2e+02) (* (Math|Vector|GetUpVector _returnvalue_3) 135.0)) _returnvalue_3 "1.000000,1.000000,1.000000") "AlwaysSpawn" "OverrideRootScale" 0 true "https://dev.app.gatevr.com/characters" 0))
      (Variables|Default|SetRef_CharSelect_HUD _returnvalue_4)
      (bind _socketioref (Variables|Default|GetSocketIoRef)
        (:then
          (EventDispatchers|BindEventtoOnLevelTravel _socketioref (EventDispatchers|CreateEvent (Variables|Default|GetRef_CharSelect_HUD) :!event DoDestroy)))
        (:else)))))

(fn ToggleWebviewHUD
  (params (IsSetURL :type Boolean) (SetURL :type String)))

(fn DeleteLaser)

(fn LoadCharacterSet
  (params (CharacterCode :type String))
  (bind _instance (CallFunction|GetGateInstance))
  (Default|SetCharacterGender _instance (NPC|CheckCharacterGender CharacterCode))
  (Default|SetCharacterCode _instance CharacterCode)
  (bind _returnvalue (Game|SpawnActorfromClass "/Game/Profile/Blueprints/BP_AssetLoad_Profile.BP_AssetLoad_Profile_C" (Math|Transform|MakeTransform "0, 0, 0" "0, 0, 0" "1.000000,1.000000,1.000000") "Undefined" "MultiplyWithRoot" 0 CharacterCode 0))
  (EventDispatchers|BindEventtoOnChracterLoadFinish _returnvalue (EventDispatchers|CreateEvent :!event SpawnNPC)))

(fn SpawnNPC
  (params (CharacterSetClass :type Character%20Preset%20Class%20Reference))
  (Default|SetCharacterPreset (CallFunction|GetGateInstance) CharacterSetClass)
  (bind _outactors (Actor|GetAllActorsOfClass "/Game/Multiplayer/Characters/Mannquin/SpawnPoint.SpawnPoint_C"))
  (Game|SpawnActorfromClass "/Game/Multiplayer/Characters/Mannquin/BP_GateCharacter_NPC.BP_GateCharacter_NPC_C" (Math|Transform|MakeTransform (.location (Transformation|GetActorTransform (Utilities|Array|Get(acopy) _outactors))) (.rotation (Transformation|GetActorTransform (Utilities|Array|Get(acopy) _outactors))) (* (.scale (Transformation|GetActorTransform (Utilities|Array|Get(acopy) _outactors))) 0.9)) "AdjustIfPossibleButAlwaysSpawn" "SelectDefaultAtRuntime" 0 CharacterSetClass 0))

(fn CheckCharacterGender
  (params (SourceString :type String))
  (return (Utilities|Enum|Equal(Enum) (Class|KismetStringLibrary|Mid SourceString 2 1) "0")))

(fn SpawnSocketIO
  (if (not (Networking|IsDedicatedServer))
    (if (Pawn|IsLocalPlayerController)
      (Variables|Default|GetSocketIoRef
        (:then)
        (:else
          (bind _returnvalue (Game|SpawnActorfromClass "/Game/CharacterSelect/Blueprints/BP_SocketIO_CharacterSelect.BP_SocketIO_CharacterSelect_C" (Math|Transform|MakeTransform "0, 0, 0" "0, 0, 0" "1.000000,1.000000,1.000000") "AlwaysSpawn" "OverrideRootScale" self 0))
          (Variables|Default|SetSocketIoRef _returnvalue)
          (CallFunction|SocketIOBindEvent))))))

(fn SetCameraPosition
  (bind _asvrpawn_login (Utilities|Casting|CastToVRPawn_Login (Pawn|GetControlledPawn)))
  (Transformation|SetRelativeLocation (Variables|/Game/VRTemplate/Blueprints/VRPawn_Login.VRPawn_Login_C|GetCamera _asvrpawn_login) "0.000000,0.000000,135.000000" false false))