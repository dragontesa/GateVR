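; Socket.IO bridge between the game and its web server, covering login, game sessions, matchmaking, user data and item events.
; On connect it binds each EventArr name to its same-named function, resends the user code if logged in and starts a ping-pong timer.
; Server handlers parse JSON and mostly fire dispatchers.
; Send functions emit requests, including base64 PNG photo uploads, and helpers load character sets and spawn NPCs.
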(event OnDisconnected(SocketIOClient)
  (params (Reason :type ESIOConnectionCloseReason%20Enum :default "CLOSE_REASON_NORMAL"))
  ;[0 0.04418 1] Connect
  ;;[1 1 1] Disconnected SocketIO / UnbindEvent
  (EventDispatchers|UnbindallEventsfromOnDisconnected (Variables|Default|GetSocketIOClient))
  (Utilities|Time|ClearandInvalidateTimerbyHandle (Variables|Timer|GetPingPongTimerHandle)))

(event OnConnected(SocketIOClient)
  (params (SocketId :type String) (SessionId :type String) (bIsReconnection :type Boolean))
  ;[0 0.04418 1] Connect
  ;;[1 1 1] Connected SocketIO / Bind Event
  (Utilities|FlowControl|Sequence
    (:then_0
      (OnConnect|OnConnectBindEvent))
    (:then_1
      (Input|EnableInput (Game|GetPlayerController 0))
      (if (Variables|/Game/Multiplayer/Blueprints/BP_GateGameInstance.BP_GateGameInstance_C|GetIsLogin (CallFunction|GetGateInstance))
        (Utilities|FlowControl|Delay 1.0)
        (SendEvent|SendUserCodeIam)))
    (:then_2
      (bind _returnvalue (Utilities|Time|SetTimerbyEvent (EventDispatchers|CreateEvent :!event SendPingPong) 2.0 true))
      (Variables|Timer|SetPingPongTimerHandle _returnvalue))))

(event Custom|s-game-start-host_Old
  (params (EventData :type SIO%20Json%20Value%20Object%20Reference))
  ;[1 1 1] Call Event
)

(event Custom|s-game-user
  (params (EventData :type SIO%20Json%20Value%20Object%20Reference))
  ;[1 1 1] Call Event
)

(event Custom|s-game-start_Old
  (params (EventData :type SIO%20Json%20Value%20Object%20Reference))
  ;[1 1 1] Call Event
)

(event Custom|UserInfo_Event
  (params (EventData :type SIO%20Json%20Value%20Object%20Reference))
  ;[1 1 1] Call Event
)

(fn ConstructionScript)

(fn JsontoValue
  (params (EventData :type SIO%20Json%20Value%20Object%20Reference) (ValueName :type String))
  (return (Class|BlueprintJsonLibrary|ToJsonValue(JsonObject) (Class|BlueprintJsonLibrary|ToJsonObject(String) (Class|SIOJsonValue|AsString EventData)) ValueName)))

(fn S-user-settings
  (params (EventData :type SIO%20Json%20Value%20Object%20Reference))
  (Default|CallOnResponseUserSetting EventData))

(fn S-response-auth
  (params (EventData :type SIO%20Json%20Value%20Object%20Reference))
  (Default|CallOnResponseSecretKey (Class|BlueprintJsonLibrary|ToString(JsonValue) (Util|JsontoValue EventData "ue_secret_key"))))

(fn EmitWebServer
  (params (EventName :type String) (Message :type SIO%20Json%20Value%20Object%20Reference))
  (Class|SocketIOClientComponent|Emit (Variables|Default|GetSocketIOClient) EventName Message "/"))

(fn EmitWebServerCallBack
  (params (EventName :type String) (Message :type SIO%20Json%20Value%20Object%20Reference) (CallbackFunctionName :type String))
  (Class|SocketIOClientComponent|EmitwithCallBack (Variables|Default|GetSocketIOClient) EventName Message CallbackFunctionName 0 "/"))

(fn SendGameExit
  (SendEvent|EmitWebServer "ue-exit-game" (Class|SIOJLibrary|ToJsonValue(String) (Variables|/Game/Multiplayer/Blueprints/BP_GateGameInstance.BP_GateGameInstance_C|GetUser_Code (CallFunction|GetGateInstance)))))

(fn SendRequestUserData
  (SendEvent|EmitWebServer "ue-req-user-data" (Class|SIOJLibrary|ToJsonValue(String) (Variables|/Game/Multiplayer/Blueprints/BP_GateGameInstance.BP_GateGameInstance_C|GetUser_Code (CallFunction|GetGateInstance)))))

(fn S-game-start-host
  (params (EventData :type SIO%20Json%20Value%20Object%20Reference))
  (Default|CallSetStartHostData true (Class|BlueprintJsonLibrary|ToString(JsonValue) (Util|JsontoValue EventData "game_id")) (Class|BlueprintJsonLibrary|ToInteger(JsonValue) (Util|JsontoValue EventData "people_count")) (Class|BlueprintJsonLibrary|ToString(JsonValue) (Util|JsontoValue EventData "game_type")) (Class|BlueprintJsonLibrary|ToString(JsonValue) (Util|JsontoValue EventData "map_name")) false))

(fn S-game-start
  (params (InputPin :type SIO%20Json%20Value%20Object%20Reference))
  (Default|CallSetStartPlayerData (Class|BlueprintJsonLibrary|ToBoolean(JsonValue) (Util|JsontoValue InputPin "is_host")) true (Class|BlueprintJsonLibrary|ToInteger(JsonValue) (Util|JsontoValue InputPin "people_count")) (Class|BlueprintJsonLibrary|ToString(JsonValue) (Util|JsontoValue InputPin "game_id")) (Class|BlueprintJsonLibrary|ToString(JsonValue) (Util|JsontoValue InputPin "fleet_id")) (Class|BlueprintJsonLibrary|ToString(JsonValue) (Util|JsontoValue InputPin "game_type")) false))

(fn SendFileUpload
  (params (Number :type Float%20%28single-precision%29) (FilePath :type String) (PhotoTakenPeople :type Array%20of%20Strings))
  (bind _returnvalue (Class|SIOJsonObject|ConstructJsonObject))
  (Utilities|FlowControl|Sequence
    (:then_0
      (Class|SIOJsonObject|SetNumberField _returnvalue "type" Number) ; 1 : image / 2 : video
    )
    (:then_1
      (Class|SIOJsonObject|SetStringField _returnvalue "s3_key" "base64") ; type : 1 일때 base64, base64가 아니면 s3 경로(video)
    )
    (:then_2
      (bind _returnvalue_2 (Game|GetCurrentLevelName true))
      (Class|SIOJsonObject|SetStringField _returnvalue "location" _returnvalue_2) ; 사진을 찍은 레벨의 이름
    )
    (:then_3
      (Class|SIOJsonObject|SetNumberField _returnvalue "is_location_code" 1.0))
    (:then_4
      (Class|SIOJsonObject|SetStringField _returnvalue "extension" "png"))
    (:then_5
      (bind _returnvalue_3 (Class|KismetRenderingLibrary|ImportFileasTexture2D FilePath))
      (Class|SIOJsonObject|SetStringField _returnvalue "base64encoded" (Utilities|String|Append "data:image/png;base64, " (Class|SIOJLibrary|Base64EncodeBytes (.OutBuffer (Class|CUBlueprintLibrary|ToBytes(Texture) _returnvalue_3 "PNG"))))))
    (:then_6
      (Class|SIOJsonObject|SetStringArrayField _returnvalue "asset_user_ids" PhotoTakenPeople))
    (:then_7
      (Class|SocketIOClientComponent|EmitwithCallBack (Variables|Default|GetSocketIOClient) "ue-asset-upload" (Class|SIOJsonValue|ConstructJsonValueObject _returnvalue) "cb_ue-asset-upload" 0 "/"))))

(fn OnConnectBindEvent
  (for _array_element (Variables|Default|GetEventArr)
    (Class|SocketIOClientComponent|BindEventtoFunction (Variables|Default|GetSocketIOClient) _array_element _array_element 0 "/" "USE_DEFAULT")))

(fn SendPingPong
  (Class|SocketIOClientComponent|Emit (Variables|Default|GetSocketIOClient) "ping" (Class|SIOJLibrary|ToJsonValue(String) (Variables|/Game/Multiplayer/Blueprints/BP_GateGameInstance.BP_GateGameInstance_C|GetUser_Code (CallFunction|GetGateInstance))) "/"))

(fn SendGameFleetID
  (params (sessionId :type String))
  (bind _returnvalue (Class|SIOJsonObject|ConstructJsonObject))
  (Class|SIOJsonObject|SetStringField _returnvalue "fleet_id" sessionId)
  (Class|SIOJsonObject|SetNumberField _returnvalue "game_id" (Math|Conversions|ToFloat(Integer) (Variables|/Game/Multiplayer/Blueprints/BP_GateGameInstance.BP_GateGameInstance_C|GetGame_ID (CallFunction|GetGateInstance))))
  (SendEvent|EmitWebServer "ue-game-fleetid" (Class|SIOJsonValue|ConstructJsonValueObject _returnvalue)))

(fn S-notifications
  (params (EventData :type SIO%20Json%20Value%20Object%20Reference))
  (Default|ToggleNotificationHUD (CallFunction|GetGateController) (Class|BlueprintJsonLibrary|ToArray(JsonValue) (Util|JsontoValue EventData "notifications"))))

(fn SendRequestAuth
  (params (UserID :type String))
  (SendEvent|EmitWebServer "ue-request-auth" (Class|SIOJLibrary|ToJsonValue(String) UserID)))

(fn S-iam
  (params (EventData :type SIO%20Json%20Value%20Object%20Reference))
  (bind _returnvalue (Util|JsontoValue EventData "is_valid"))
  (bind _returnvalue_2 (Class|BlueprintJsonLibrary|ToBoolean(JsonValue) _returnvalue))
  (Default|CallCallonPlayLoginResultSound _returnvalue_2)
  (if _returnvalue_2
    (Default|CallOnTryLogin)
    (SendEvent|SendRequestAuth (Variables|/Game/Multiplayer/Blueprints/BP_GateGameInstance.BP_GateGameInstance_C|GetUser_Code (CallFunction|GetGateInstance)))
    (else
      (Default|CallOnLoginFailed))))

(fn S-resp-user-data
  (params (InputPin :type SIO%20Json%20Value%20Object%20Reference))
  (Default|CallOnResponseUserData (Utilities|Struct|MakeFPlayer_NameTag (Class|BlueprintJsonLibrary|ToString(JsonValue) (Util|JsontoValue InputPin "user_name")) (Class|BlueprintJsonLibrary|ToString(JsonValue) (Util|JsontoValue InputPin "user_profile_url")) 0 "NewEnumerator0")))

(fn SendUserCodeIam
  (SendEvent|EmitWebServer "iam" (Class|SIOJLibrary|ToJsonValue(Integer) (Math|Conversions|ToInteger(Byte) (Variables|/Game/Multiplayer/Blueprints/BP_GateGameInstance.BP_GateGameInstance_C|GetUser_Code (CallFunction|GetGateInstance))))))

(fn SendReqUserSetting
  (SendEvent|EmitWebServer "req-user-settings" (Class|SIOJLibrary|ToJsonValue(Integer) (Math|Conversions|ToInteger(Byte) (Variables|/Game/Multiplayer/Blueprints/BP_GateGameInstance.BP_GateGameInstance_C|GetUser_Code (CallFunction|GetGateInstance))))))

(fn SendReqUserInfo
  (SendEvent|EmitWebServer "ue-req-user-info"))

(fn S-error
  (Default|CallOnLoginFailed))

(fn S-exit-page
  (Default|CallCloseSetting))

(fn CbUe-asset-upload
  (params (Input :type SIO%20Json%20Value%20Object%20Reference)))

(fn SendJoin-dedicate
  (SendEvent|EmitWebServer "join-dedicate" (Class|SIOJLibrary|ToJsonValue(String) (Variables|/Game/Multiplayer/Blueprints/BP_GateGameInstance.BP_GateGameInstance_C|GetUser_Code (CallFunction|GetGateInstance)))))

(fn SendExit-dedicate
  (SendEvent|EmitWebServer "exit-dedicate" (Class|SIOJLibrary|ToJsonValue(String) (Variables|/Game/Multiplayer/Blueprints/BP_GateGameInstance.BP_GateGameInstance_C|GetUser_Code (CallFunction|GetGateInstance)))))

(fn Dedicate-start
  (params (EventData :type SIO%20Json%20Value%20Object%20Reference))
  (if (Utilities|Enum|Equal(Enum) (Variables|/Game/Multiplayer/Blueprints/BP_GateGameInstance.BP_GateGameInstance_C|GetUser_Code (CallFunction|GetGateInstance)) (Class|BlueprintJsonLibrary|ToString(JsonValue) (Util|JsontoValue EventData "host_code")))
    (Default|CallTravelDediServer (Class|BlueprintJsonLibrary|ToString(JsonValue) (Util|JsontoValue EventData "map_name")))
    (Variables|/Game/Multiplayer/Blueprints/BP_GateGameInstance.BP_GateGameInstance_C|SetIsHost (CallFunction|GetGateInstance) true)
    (else
      (Variables|/Game/Multiplayer/Blueprints/BP_GateGameInstance.BP_GateGameInstance_C|SetIsHost (CallFunction|GetGateInstance) false))))

(fn S-matching-move-room
  (params (EventData :type SIO%20Json%20Value%20Object%20Reference))
  (Default|CallJoinMatchServer (Class|BlueprintJsonLibrary|ToString(JsonValue) (Util|JsontoValue EventData "gamesession_id"))))

(fn S-matching-change-map
  (params (EventData :type SIO%20Json%20Value%20Object%20Reference))
  (if (Variables|/Game/Multiplayer/Blueprints/BP_GateGameInstance.BP_GateGameInstance_C|GetIsHost (CallFunction|GetGateInstance))
    (Default|CallTravelDediServer (Class|BlueprintJsonLibrary|ToString(JsonValue) (Util|JsontoValue EventData "map_name")))))

(fn S-web-login-success
  (params (InputPin :type SIO%20Json%20Value%20Object%20Reference))
  (Default|CallOnLevelTravel)
  (Default|CallOnSignedinSuccessfully))

(fn S-item-changed
  (params (Input :type SIO%20Json%20Value%20Object%20Reference))
  (Default|CallItemChanged (Class|BlueprintJsonLibrary|ToString(JsonValue) (Util|JsontoValue Input "item_code")) (Class|BlueprintJsonLibrary|ToBoolean(JsonValue) (Util|JsontoValue Input "wear")))
  (Development|PrintString "Call S-Item-Changed" true true "(R=0.000000,G=0.660000,B=1.000000,A=1.000000)" 1e+01))

(fn S-item-entered
  (params (Input :type SIO%20Json%20Value%20Object%20Reference))
  (Default|CallIsEnterItemCategory true))

(fn S-item-exited
  (params (Input :type SIO%20Json%20Value%20Object%20Reference))
  (Default|CallIsEnterItemCategory false))

(fn S-mirror-turn-on
  (params (Input :type SIO%20Json%20Value%20Object%20Reference))
  (Default|CallIsEnterItemCategory true)
  (Development|PrintString "S-mirror-turn-on" true true "(R=1.000000,G=0.000000,B=0.000000,A=1.000000)" 1e+01))

(fn S-mirror-turn-off
  (params (Input :type SIO%20Json%20Value%20Object%20Reference))
  (Default|CallIsEnterItemCategory false))

(fn S-item-clicked
  (params (Input :type SIO%20Json%20Value%20Object%20Reference))
  (Default|CallItemPartsClicked (Class|SIOJsonValue|AsString Input)))

(fn S-game-user-enter
  (params (Input :type SIO%20Json%20Value%20Object%20Reference))
  (if (Utilities|Enum|Equal(Enum) (Class|BlueprintJsonLibrary|ToString(JsonValue) (Util|JsontoValue Input "user_id")) (Variables|/Game/Multiplayer/Blueprints/BP_GateGameInstance.BP_GateGameInstance_C|GetUser_Id (CallFunction|GetGateInstance)))
    (Default|CallOnEnterGameReadyRoom true (Class|BlueprintJsonLibrary|ToString(JsonValue) (Util|JsontoValue Input "game_id")))
    (Development|PrintString "S-game-user-enter" true true "(R=1.000000,G=0.000000,B=0.000000,A=1.000000)" 1e+01)))

(fn S-game-user-exit
  (params (Input :type SIO%20Json%20Value%20Object%20Reference))
  (if (Utilities|Enum|Equal(Enum) (Class|BlueprintJsonLibrary|ToString(JsonValue) (Util|JsontoValue Input "user_id")) (Variables|/Game/Multiplayer/Blueprints/BP_GateGameInstance.BP_GateGameInstance_C|GetUser_Id (CallFunction|GetGateInstance)))
    (Default|CallOnEnterGameReadyRoom false (Class|BlueprintJsonLibrary|ToString(JsonValue) (Util|JsontoValue Input "game_id")))
    (Development|PrintString "S-game-user-exit" true true "(R=1.000000,G=0.000000,B=0.000000,A=1.000000)" 1e+01)))

(fn S-change-character
  (params (EventData :type SIO%20Json%20Value%20Object%20Reference))
  (Default|CallOnEnterCharacterSelect))

(fn S-game-exit
  (params (EventData :type SIO%20Json%20Value%20Object%20Reference))
  (Default|CallOnEnterWorld))

(fn LoadCharacterSet
  (params (CharacterCode :type String))
  (Default|SetCharacterGender (CallFunction|GetGateInstance) (Utilities|Enum|Equal(Enum) (Class|KismetStringLibrary|Mid CharacterCode 2 1) "0"))
  (bind _returnvalue (Game|SpawnActorfromClass "/Game/Profile/Blueprints/BP_AssetLoad_Profile.BP_AssetLoad_Profile_C" (Math|Transform|MakeTransform "0, 0, 0" "0, 0, 0" "1.000000,1.000000,1.000000") "Undefined" "MultiplyWithRoot" 0 CharacterCode 0))
  (EventDispatchers|BindEventtoOnChracterLoadFinish _returnvalue (EventDispatchers|CreateEvent :!event SpawnNPC)))

(fn SpawnNPC
  (params (CharacterSetClass :type Character%20Preset%20Class%20Reference))
  (Default|SetCharacterPreset (CallFunction|GetGateInstance) CharacterSetClass)
  (bind _outactors (Actor|GetAllActorsOfClass "/Game/Multiplayer/Characters/Mannquin/SpawnPoint.SpawnPoint_C"))
  (Game|SpawnActorfromClass "/Game/Multiplayer/Characters/Mannquin/BP_GateCharacter_NPC.BP_GateCharacter_NPC_C" (Math|Transform|MakeTransform (.location (Transformation|GetActorTransform (Utilities|Array|Get(acopy) _outactors))) (.rotation (Transformation|GetActorTransform (Utilities|Array|Get(acopy) _outactors))) (* (.scale (Transformation|GetActorTransform (Utilities|Array|Get(acopy) _outactors))) 0.9)) "AdjustIfPossibleButAlwaysSpawn" "SelectDefaultAtRuntime" 0 CharacterSetClass 0))