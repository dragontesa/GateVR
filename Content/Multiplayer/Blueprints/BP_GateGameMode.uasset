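; Multiplayer game mode for Gate that manages player login, spawning, logout and lobby teardown, with GameLift session handling.
; Login registers controllers and caches PlayerStarts; respawn spawns a PC or VR character at a random unoccupied start and adds a name tag.
; Logout releases GameLift player sessions; when the last player leaves, it ends the game session and server-travels to the default map.
; Requested travel notifies controllers, starts a timer and suppresses that GameLift cleanup.
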(event Custom|TearDownLobby
  ;[0.1329 0.1912 0.2705] Tear down lobby and travel to the server default
  (CallFunction|FinishGameLiftGameSession)
  (CallFunction|ReleaseTalkingFree)
  (Utilities|FlowControl|Delay 1.0)
  (Development|ExecuteConsoleCommand "servertravel GameLift_ServerDefault" 0))

(event Custom|RespawnPlayer
  (params (Controller :type Player%20Controller%20Object%20Reference) (Character :type Character%20Preset%20Class%20Reference) (IsHost :type Boolean) (IsDesktop :type Boolean))
  ;[0.246 0.2285 1] Spawn the players as base character when arriving at the Lobby Menu / Tells everyone to update their Lobby
  (SpawnCharacter|DestroyOldCharacter Controller)
  (bind _returnvalue (Game|SpawnActorfromClass (.AsBP%20Gate%20Character%20VR (Utilities|Casting|CastToBP_GateCharacter_VRClass (Class|KismetMathLibrary|SelectClass "/Game/Multiplayer/Characters/BP_GateCharacter_PC.BP_GateCharacter_PC_C" "/Game/Multiplayer/Characters/FBIK/BP_GateCharacter_VR.BP_GateCharacter_VR_C" IsDesktop))) (Transformation|GetActorTransform (SpawnCharacter|GetRandomSpawnPoint Controller IsHost)) "AlwaysSpawn" "SelectDefaultAtRuntime" 0 Character 0))
  (Pawn|Possess Controller _returnvalue)
  (NameTag|SpawnNameTag Controller))

(event Custom|RemovePlayer
  (params (RemovalPlayer :type Player%20Controller%20Object%20Reference))
  (bind _allplayercontrollers (Variables|Players|GetAllPlayerControllers))
  ;[0.1329 0.1912 0.2705] Remove The Logout Player Controller in the List
  (Utilities|Array|RemoveItem _allplayercontrollers RemovalPlayer)
  (if (and (<= (Utilities|Array|Length _allplayercontrollers) 0) (not (Variables|ServerTravel|GetIsServertravel)))
    (CallFunction|TearDownLobby)))

(event EventPostLogin
  (params (NewPlayer :type Player%20Controller%20Object%20Reference))
  ;[0.06828 1 0.1242] Spawn new player and Setup Lobby Menu on Post Login on Server Side
  (Utilities|FlowControl|Sequence
    (:then_0
      (Utilities|Array|Add (Variables|Players|GetAllPlayerControllers) NewPlayer)
      (bind _outactors (Actor|GetAllActorsOfClass "/Script/Engine.PlayerStart"))
      (Variables|SpawnCharacter|SetSpawnPoints _outactors))
    (:then_1
      (bind _asbp_gate_player_controller (Utilities|Casting|CastToBP_GatePlayerController NewPlayer))
      (Default|InitialSetup _asbp_gate_player_controller))
    (:then_2
      (Default|CallOnPostLogin))))

(event EventOnLogout
  (params (ExitingController :type Controller%20Object%20Reference))
  ;[1 1 1] Logout
  (bind _asbp_gate_player_controller (Utilities|Casting|CastToBP_GatePlayerController ExitingController))
  (Utilities|FlowControl|Sequence
    (:then_0
      (if (not (Variables|ServerTravel|GetIsServertravel))
        (CallFunction|LogoutGameLiftPlayer (Variables|/Game/Multiplayer/Blueprints/BP_GatePlayerController.BP_GatePlayerController_C|GetGameLiftPlayerSessionId _asbp_gate_player_controller)) ; Logout GameLift Player, If does not GameLift Player, then just nothing
      ))
    (:then_1
      (CallFunction|RemovePlayer _asbp_gate_player_controller))
    (:then_2
      (Default|CallOnPostLogout))))

(event EventBeginPlay
  (DeadZone|SpawnDeadZone))

(fn ConstructionScript)

(fn SpawnDeadZone
  (bind _returnvalue (Game|SpawnActorfromClass "/Game/Multiplayer/Blueprints/BP_RespawnCollision.BP_RespawnCollision_C" (Math|Transform|MakeTransform "0.000000,0.000000,-15000.000000" "0, 0, 0" "1.000000,1.000000,1.000000") "AlwaysSpawn" "OverrideRootScale" 0 0))
  (Variables|DeadZone|SetRef_RespawnCollision _returnvalue))

(fn SpawnCalibratePopup
  (bind _controller (CallFunction|GetGateController))
  (bind _instance (CallFunction|GetGateInstance))
  (if (not (Variables|/Game/Multiplayer/Blueprints/BP_GateGameInstance.BP_GateGameInstance_C|GetIsCalibrateGuided _instance))
    (Variables|/Game/Multiplayer/Blueprints/BP_GateGameInstance.BP_GateGameInstance_C|SetIsCalibrateGuided _instance true)
    (Utilities|IsValid _controller
      (:Is%20Valid
        (Default|ToggleCalibrateHUD _controller)))))

(fn DestroyOldCharacter
  (params (Controller :type Controller%20Object%20Reference))
  (bind _returnvalue (Pawn|GetControlledPawn Controller))
  (Utilities|IsValid _returnvalue
    (:Is%20Valid
      (Actor|DestroyActor _returnvalue))))

(fn GetRandomSpawnPoint
  (params (SpawnPlayerController :type Player%20Controller%20Object%20Reference) (IsHost :type Boolean))
  (bind _spawnpoints (Variables|SpawnCharacter|GetSpawnPoints))
  (bind _availablepoints (LocalVariables|GetAvailablePoints))
  (bind _returnvalue (Utilities|Array|Length _availablepoints))
  (for _array_element (Variables|SpawnCharacter|GetSpawnPoints)
    (if (not (SpawnCharacter|IsOverlapingPlayer _array_element))
      (Utilities|Array|Add (LocalVariables|GetAvailablePoints) _array_element)))
  (return (select (> _returnvalue 0) (Utilities|Array|Get(acopy) _availablepoints (Math|Random|RandomInteger _returnvalue)) (Utilities|Array|Get(acopy) _spawnpoints (Math|Random|RandomInteger (Utilities|Array|Length _spawnpoints))))))

(fn SpawnNameTag
  (params (Controller :type Player%20Controller%20Object%20Reference))
  (bind (_playerstate _success) (CallFunction|GetGateStatebyController Controller))
  (if _success
    (Default|SpawnPersonalStateUI _playerstate Controller)))

(fn RequestServerTravel
  (params (MapName :type String))
  (Variables|/Game/Multiplayer/Blueprints/BP_GateGameInstance.BP_GateGameInstance_C|SetUserCount (CallFunction|GetGateInstance) (Utilities|Array|Length (Variables|Players|GetAllPlayerControllers)))
  (Variables|ServerTravel|SetIsServertravel true)
  (ServerTravel|PrevServerTravel)
  (Utilities|Time|SetTimerbyEvent (EventDispatchers|CreateEvent :!event StartServerTravel) 5.0))

(fn IsOverlapingPlayer
  (params (Actor :type Actor%20Object%20Reference))
  (bind _outactors (Actor|GetAllActorsOfClass "/Game/Multiplayer/Characters/FBIK/BP_GateCharacter_VR.BP_GateCharacter_VR_C"))
  (bind _array_element (Utilities|Array|ForEachLoopwithBreak _outactors :!label _label)
    (:LoopBody
      (bind _output_get (LocalVariables|SetOverlaped (< (Math|Vector|VectorLengthXY (- (Transformation|GetActorLocation _array_element) (Transformation|GetActorLocation Actor))) (LocalVariables|GetOverlapDistance))))
      (if _output_get
        (goto _label Break)))
    (:Completed
      (return (LocalVariables|GetOverlaped)))))

(fn PrevServerTravel
  (for _array_element (Variables|Players|GetAllPlayerControllers)
    (bind _asbp_gate_player_controller (Utilities|Casting|CastToBP_GatePlayerController _array_element))
    (Default|PrevServerTravelOwn _asbp_gate_player_controller)))

(fn StartServerTravel
  (Development|ExecuteConsoleCommand "servertravel GameLift_ServerDefault" 0))