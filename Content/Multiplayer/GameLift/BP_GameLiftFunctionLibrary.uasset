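; Blueprint function library wrapping AWS GameLift session management for multiplayer.
; It lazily creates and caches a GameLift client on the Gate instance, initialized with hard-coded AWS credentials and SSL verification off, to create lobby game sessions and random-ID player sessions.
; Helpers open the server address with the player session ID, trigger game-mode travel, and remove or finish sessions.
; Others save and load player info via a save slot and detect GameLift from command-line flags.
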(fn InitGameLift
  (bind _instance (CallFunction|GetGateInstance))
  (bind _gategameliftref (Variables|/Game/Multiplayer/Blueprints/BP_GateGameInstance.BP_GateGameInstance_C|GetGateGameLiftRef _instance)
    (:then
      (return _gategameliftref))
    (:else
      (bind _gameliftactor (Default|SpawnGateGameLift _instance))
      (bind _output_get (Variables|/Game/Multiplayer/Blueprints/BP_GateGameInstance.BP_GateGameInstance_C|SetGateGameLiftRef (CallFunction|GetGateInstance) _gameliftactor))
      (Class|GateGameLiftClient|Init _output_get (Utilities|Struct|MakeGameLiftClientData (Utilities|Struct|MakeAWSCredentials "AKIAXCWALYIRMDVIF4KC" "JpVCV8wVzKzdqlATbep2DXgQtktFdSdXYZtoRu1P" "" "0001.01.01-00.00.00") (Utilities|Struct|MakeAWSClientConfiguration "" "https" "ap-northeast-2" false false 25 0 3000 1000 true 30 1 "" "http" "" 0 "" "" "" "" "" "" "" 0 false)))
      (return _output_get))))

(fn StartGameSession
  (bind _instance (CallFunction|GetGateInstance))
  (bind _gategameliftref (Variables|/Game/Multiplayer/Blueprints/BP_GateGameInstance.BP_GateGameInstance_C|GetGateGameLiftRef _instance))
  (Class|GateGameLiftClient|CreateGameSession _gategameliftref (Utilities|Struct|MakeCreateGameSessionRequest (Variables|/Script/GateGameLift.GateGameLiftClient|GetFleetId _gategameliftref) 10 "Lobby")))

(fn StartPlayer
  (bind _gategameliftref (Variables|/Game/Multiplayer/Blueprints/BP_GateGameInstance.BP_GateGameInstance_C|GetGateGameLiftRef (CallFunction|GetGateInstance))
    (:then
      (Class|GateGameLiftClient|CreatePlayerSession _gategameliftref (Utilities|Struct|MakeCreatePlayerSessionRequest (Variables|/Script/GateGameLift.GateGameLiftClient|GetGameSessionId _gategameliftref) (Utilities|Struct|BreakAWSUUID (Class|UUID|RandomUUID)))))
    (:else)))

(fn ConnectGameServer
  (params (PlayerSessionId :type String) (IpAddress :type String) (PortNum :type Integer) (LevelName :type String) (Absolute :type Boolean))
  (Game|OpenLevel(byName) 0 (Utilities|String|StringToName (Utilities|String|Append IpAddress ":" (Utilities|String|ToString(Integer) PortNum))) Absolute (Utilities|String|Append "PlayerSessionId=" PlayerSessionId)))

(fn StartTravelIntoGame
  (bind _asbp_game_lift_server_game_mode (Utilities|Casting|CastToBP_GameLift_ServerGameMode (Game|GetGameMode)))
  (Default|TravelGame _asbp_game_lift_server_game_mode))

(fn SaveGameLiftPlayerInfo
  (params (GameliftPlayerinfo :type BP%20Game%20Lift%20Player%20Info%20Structure))
  (bind _playersavegameref (Variables|/Game/Multiplayer/Blueprints/BP_GateGameInstance.BP_GateGameInstance_C|GetPlayerSaveGameRef (CallFunction|GetGateInstance))
    (:then
      (LocalVariables|SetPlayerSaveGameRef _playersavegameref))
    (:else
      (bind _returnvalue (SaveGame|CreateSaveGameObject "/Game/Multiplayer/Blueprints/BP_PlayerSaveGameMP.BP_PlayerSaveGameMP_C"))
      (LocalVariables|SetPlayerSaveGameRef _returnvalue)))
  (Variables|/Game/Multiplayer/Blueprints/BP_PlayerSaveGameMP.BP_PlayerSaveGameMP_C|SetS_GameLiftPlayerInfo (LocalVariables|GetPlayerSaveGameRef) GameliftPlayerinfo)
  (SaveGame|SaveGametoSlot (LocalVariables|GetPlayerSaveGameRef) "PlayerSettingsSave"))

(fn LoadGameLiftPlayerInfo
  (bind _returnvalue (SaveGame|LoadGamefromSlot "PlayerSettingsSave"))
  (bind _asbp_player_save_game_mp (Utilities|Casting|CastToBP_PlayerSaveGameMP _returnvalue)
    (:then
      (|SetBy-RefVar (LocalVariables|GetLoadGameliftPlayerInfo) (Variables|/Game/Multiplayer/Blueprints/BP_PlayerSaveGameMP.BP_PlayerSaveGameMP_C|GetS_GameLiftPlayerInfo _asbp_player_save_game_mp))
      (return (LocalVariables|GetLoadGameliftPlayerInfo)))
    (:CastFailed
      (return (LocalVariables|GetLoadGameliftPlayerInfo)))))

(fn LogoutGameLiftPlayer
  (params (PlayerSessionId :type String))
  (bind _returnvalue (Class|GateGameLiftServerWrapper|RemovePlayerSession PlayerSessionId))
  (return _returnvalue))

(fn FinishGameLiftGameSession
  (params (GameLiftGameSessionId :type String))
  (Class|GateGameLiftServerWrapper|FinishGameSession))

(fn IsGameLiftEnabled
  (bind _returnvalue (Utilities|GetCommandLine))
  (return (or (Utilities|String|Contains _returnvalue "WithGameLift") (Utilities|String|Contains _returnvalue "fleet"))))