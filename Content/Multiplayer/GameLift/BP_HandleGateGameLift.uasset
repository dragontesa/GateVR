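; Gate-side GameLift handler that creates game and player sessions and connects the player to the game server.
; BeginPlay binds both creation callbacks and passes the gate instance's session ID and user count into its own state.
; Game session success broadcasts the ID; player session success saves GameLift info, releases voice, fades and connects after a delay.
; Test events trigger each creation manually; an older online-session create/destroy path is disabled.
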(event Custom|Test_CreateGameSession
  ;[0.1329 0.1912 0.2705] Touring GameLift Session
  (EventDispatchers|BindEventtoOnGameSessionCreated (EventDispatchers|CreateEvent :!event Custom|HandleOnGameSessionCreated))
  (CallFunction|StartGameSession))

(event Custom|Test_CreatePlayerSession
  ;[0.1329 0.1912 0.2705] Start GameLift Player
  (EventDispatchers|BindEventtoOnPlayerSessionCreated (EventDispatchers|CreateEvent :!event Custom|HandleOnPlayerSessionCreated))
  (CallFunction|StartPlayer))

(event Custom|HandleOnGameSessionCreated
  (params (success :type Boolean) (GameSessionId :type String))
  ;[0.1329 0.1912 0.2705] Send Game Session Id to Web Server
  (if success
    (Default|CallOnCreateGameSessionSuccess GameSessionId)))

(event Custom|HandleOnPlayerSessionCreated
  (params (success :type Boolean) (PlayerSessionId :type String) (IpAddress :type String) (PortNumber :type Integer))
  ;[0.1329 0.1912 0.2705] GameLift Player Session Id Creation and Connect to Game Server with the Player Session ID
  (if success
    (Default|CallOnCreatePlayerSessionSuccess)
    (CallFunction|SavePlayerInfo PlayerSessionId)
    (Default|ReleaseVoice (CallFunction|GetGateInstance))
    (Default|Fadein (CallFunction|GetGateController))
    (Utilities|FlowControl|Delay 5.0)
    (CallFunction|ConnectGameServer PlayerSessionId IpAddress PortNumber "" (not (Class|KismetSystemLibrary|IsStandalone)))))

(event EventBeginPlay
  (bind _instance (CallFunction|GetGateInstance))
  (EventDispatchers|BindEventtoOnGameSessionCreated (EventDispatchers|CreateEvent :!event Custom|HandleOnGameSessionCreated))
  (EventDispatchers|BindEventtoOnPlayerSessionCreated (EventDispatchers|CreateEvent :!event Custom|HandleOnPlayerSessionCreated))
  (Class|GateGameLiftClient|SetisfyGameSession (Variables|/Game/Multiplayer/Blueprints/BP_GateGameInstance.BP_GateGameInstance_C|GetGamesession_ID _instance))
  (Variables|Default|SetPlayerNumbers (Variables|/Game/Multiplayer/Blueprints/BP_GateGameInstance.BP_GateGameInstance_C|GetUserCount _instance)))

(fn ConstructionScript)

(fn SavePlayerInfo
  (params (Player_PlayerSessionID :type String))
  (CallFunction|SaveGameLiftPlayerInfo (Utilities|Struct|MakeBP_GameLift_PlayerInfo (Variables|Default|GetGameSessionId) Player_PlayerSessionID (Variables|Default|GetFleetId) false)))