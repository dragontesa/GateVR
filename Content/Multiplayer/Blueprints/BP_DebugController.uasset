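; BP_DebugController is a debug controller for multiplayer that adds a third-person toggle on the VRIK reference, bound to debug key NumPad 9.
; StartLevelLoad only calls RevertSystemBlock, and BeginVoice is an empty override that leaves the parent's voice setup uncalled.
; A hard-coded UserID and socket user-code send remain in the event graph but never run.
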(event EventBeginPlay
  (|CallParentFunction))

(event Input|KeyboardEvents|DebugKeyNumPadNine
  (params (Key :type Key%20Structure :default "None") (ActionValue :type Input%20Action%20Value%20Structure))
  (:Pressed
    (bind _ref_vrik (Variables|Default|GetRef_VRIK)
      (:then
        (Default|ToggleThirdPerson _ref_vrik))
      (:else))))

(fn ConstructionScript
  (|CallParentFunction))

(fn StartLevelLoad
  (CallFunction|RevertSystemBlock))

(fn BeginVoice)